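; BP_MissileExplosion is a missile explosion actor that plays a sound on spawn and damages enemies it collides with.
; Each tick it shrinks its explosion mesh, destroying itself once the scale would drop below zero.
; An ignored-enemies list limits damage to one hit per enemy, while empty overrides bypass the parent's world and bullet collision handling.
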(event EventTick
  (params (DeltaSeconds :type Float%20%28single-precision%29))
  (bind _explosionmesh (Variables|Default|GetExplosionMesh))
  (bind _shrinkrate (Variables|Default|GetShrinkRate))
  (bind _returnvalue (* DeltaSeconds _shrinkrate))
  (bind _relativescale3d (Variables|/Script/Engine.SceneComponent|GetRelativeScale3D _explosionmesh))
  (bind _returnvalue_2 (- _relativescale3d _returnvalue))
  (Transformation|SetRelativeScale3D _explosionmesh _returnvalue_2)
  (if (< (.X (Math|Vector|BreakVector _returnvalue_2)) 0.0)
    (Actor|DestroyActor)))

(event EventEventCollideEnemy
  (params (Enemy :type BP%20Enemy%20Object%20Reference))
  (if (not (Utilities|Array|ContainsItem (Variables|Default|GetIgnoredEnemies) Enemy))
    (Game|Damage|ApplyDamage Enemy (Variables|Default|GetDamage) 0 0 (Variables|Default|GetDamageType))
    (Utilities|Array|Add (Variables|Default|GetIgnoredEnemies) Enemy)))

(event EventBeginPlay
  (Audio|PlaySoundatLocation (Variables|Default|GetExplosionSound) (Transformation|GetActorLocation)))

(event EventEventCollideWorld)

(event EventEventCollideBullet)

(fn ConstructionScript
  (|CallParentFunction))