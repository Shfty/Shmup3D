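; BP_ShockBlast is a player projectile that acts as an instant, piercing beam rather than a moving shot.
; On BeginPlay, a forward visibility trace ignoring the player sets the beam's length, and the actor shifts to its midpoint.
; Tick shrinks the beam's width until it destroys itself.
; Each enemy touched takes damage once and triggers game-state hitstop, while bullet and world collisions do nothing.
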(event EventTick
  (params (DeltaSeconds :type Float%20%28single-precision%29))
  (bind _shrinkrate (Variables|Default|GetShrinkRate))
  (bind _rootscene (Variables|Default|GetRootScene))
  (bind _returnvalue (* DeltaSeconds _shrinkrate))
  (bind _relativescale3d (Variables|/Script/Engine.SceneComponent|GetRelativeScale3D _rootscene))
  (bind _returnvalue_2 (- _relativescale3d _returnvalue))
  (bind (_x _y) (Math|Vector|BreakVector _returnvalue_2))
  (Transformation|SetRelativeScale3D _rootscene (Math|Vector|MakeVector _x _y (Math|Float|Max(Float) (.Z (Math|Vector|BreakVector _relativescale3d)) 0.001)))
  (if (<= (.X (Math|Vector|BreakVector _returnvalue_2)) 0.0)
    (Actor|DestroyActor)))

(event EventCollideEnemy
  (params (Enemy :type BP%20Enemy%20Object%20Reference))
  (bind _damagetype (Variables|Default|GetDamageType))
  (if (not (Utilities|Array|ContainsItem (Variables|Default|GetIgnoredEnemies) Enemy))
    (Game|Damage|ApplyDamage Enemy (Variables|Default|GetDamage) 0 0 _damagetype)
    (Utilities|Array|Add (Variables|Default|GetIgnoredEnemies) Enemy)
    (Default|EventHitstop (CallFunction|GetGameState) (Utilities|GetClassDefaults _damagetype))))

(event EventBeginPlay
  (bind _returnvalue (Transformation|GetActorLocation))
  (bind _rootscene (Variables|Default|GetRootScene))
  (bind _relativescale3d (Variables|/Script/Engine.SceneComponent|GetRelativeScale3D _rootscene))
  (bind _outhit (Collision|LineTraceByChannel _returnvalue (+ _returnvalue (* (Transformation|GetActorForwardVector) (Variables|Default|GetMaxTraceDistance))) "TraceTypeQuery1" false (Utilities|Array|MakeArray (Game|Player|GetPlayerPawn 0)) "None"))
  (Transformation|SetRelativeScale3D _rootscene (Math|Vector|MakeVector (.x _relativescale3d) (.y _relativescale3d) (* (* (.Time (Collision|BreakHitResult _outhit)) (Variables|Default|GetMaxTraceDistance)) 0.01)))
  (Transformation|AddActorLocalOffset (Math|Vector|MakeVector (* (* (.Time (Collision|BreakHitResult _outhit)) (Variables|Default|GetMaxTraceDistance)) 0.5) 0.0 0.0) false true)
  (|CallParentFunction))

(event EventCollideWorld)

(event EventCollideBullet)

(fn ConstructionScript
  (|CallParentFunction))