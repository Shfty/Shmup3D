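; Player missile projectile that speeds up in flight and explodes when it hits an enemy or the world.
; Tick adds forward-vector Acceleration, scaled by delta time, to the ProjectileMovement velocity.
; Enemy and world collisions spawn BP_MissileExplosion, flagged to move relative to the play volume, then defer to parent handling.
; The bullet collision override is empty and skips parent handling, so the missile does not react to bullets.
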(event EventTick
  (params (DeltaSeconds :type Float%20%28single-precision%29))
  (bind _projectilemovement (Variables|Default|GetProjectileMovement))
  (Variables|/Script/Engine.MovementComponent|SetVelocity _projectilemovement (+ (Variables|/Script/Engine.MovementComponent|GetVelocity _projectilemovement) (* (* (Transformation|GetActorForwardVector) (Variables|Default|GetAcceleration)) DeltaSeconds))))

(event EventEventCollideEnemy
  (params (Enemy :type BP%20Enemy%20Object%20Reference))
  (Game|SpawnActorfromClass "/Game/Blueprints/Player/Projectiles/BP_MissileExplosion.BP_MissileExplosion_C" (Transformation|GetActorTransform) "AlwaysSpawn" 0 true 0)
  (|CallParentFunction Enemy))

(event EventEventCollideWorld
  (Game|SpawnActorfromClass "/Game/Blueprints/Player/Projectiles/BP_MissileExplosion.BP_MissileExplosion_C" (Transformation|GetActorTransform) "AlwaysSpawn" 0 true 0)
  (|CallParentFunction))

(event EventEventCollideBullet)

(fn ConstructionScript
  (|CallParentFunction))