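; BP_MiniBlast is a player projectile Blueprint that inherits its behavior from a parent class.
; Its only active custom logic overrides the bullet collision event, deactivating the ParticleHitbox and DamageHitbox components before passing the event on to the parent.
; The construction script just calls the parent, and the BeginPlay, Tick and overlap events are unused disabled stubs.
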(event EventBeginPlay
  (|CallParentFunction))

(event Collision|EventActorBeginOverlap
  (params (OtherActor :type Actor%20Object%20Reference)))

(event EventTick
  (params (DeltaSeconds :type Float%20%28single-precision%29))
  (|CallParentFunction 0.0))

(event EventEventCollideBullet
  (Components|Activation|Deactivate (Variables|Default|GetParticleHitbox))
  (Components|Activation|Deactivate (Variables|Default|GetDamageHitbox))
  (|CallParentFunction))

(fn ConstructionScript
  (|CallParentFunction))