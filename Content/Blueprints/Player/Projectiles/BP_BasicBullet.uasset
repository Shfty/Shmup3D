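; Basic player bullet projectile that homes in on a TargetEnemy when one is set.
; On BeginPlay with a valid target, it zeroes projectile movement and caches its start location.
; Each Tick, it sweeps itself along the line from that start toward the target's current position, using accumulated distance at TravelSpeed.
; If a locked target becomes invalid, it restores projectile movement and flies along its forward vector.
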(event EventBeginPlay
  (Utilities|FlowControl|Sequence
    (:then_0
      (Utilities|IsValid (Variables|Default|GetTargetEnemy)
        (:Is%20Valid
          (CallFunction|DisableProjectileMovement)
          (Variables|Default|SetCachedStartLocation (Transformation|GetActorLocation))
          (Variables|Default|SetbLockedOn true))))
    (:then_1
      (|CallParentFunction))))

(event EventTick
  (params (DeltaSeconds :type Float%20%28single-precision%29))
  (bind _cachedstartlocation (Variables|Default|GetCachedStartLocation))
  (bind _targetenemy (Variables|Default|GetTargetEnemy))
  (bind _returnvalue (Transformation|GetActorLocation _targetenemy))
  (bind _returnvalue_2 (- _returnvalue _cachedstartlocation))
  (bind _returnvalue_3 (Math|Vector|Normalize _returnvalue_2))
  (Utilities|IsValid (Variables|Default|GetTargetEnemy)
    (:Is%20Valid
      (Variables|Default|SetDistanceTraveled (+ (Variables|Default|GetDistanceTraveled) (* DeltaSeconds (Variables|Default|GetTravelSpeed))))
      ;[1 1 1] Comment
      (Transformation|SetActorLocationAndRotation (+ _cachedstartlocation (* _returnvalue_3 (Variables|Default|GetDistanceTraveled))) (Math|Rotator|MakeRotfromX _returnvalue_3) true))
    (:Is%20Not%20Valid
      (if (Variables|Default|GetbLockedOn)
        (CallFunction|EnableProjectileMovement)
        (Variables|/Script/Engine.MovementComponent|SetVelocity (Variables|Default|GetProjectileMovement) (* (Transformation|GetActorForwardVector) (Variables|Default|GetTravelSpeed)))))))

(event EventCollideBullet)

(fn ConstructionScript
  (CallFunction|EnableProjectileMovement)
  (|CallParentFunction))

(fn EnableProjectileMovement
  (bind _projectilemovement (Variables|Default|GetProjectileMovement))
  (bind _travelspeed (Variables|Default|GetTravelSpeed))
  (Variables|/Script/Engine.ProjectileMovementComponent|SetMaxSpeed _projectilemovement _travelspeed)
  (Variables|/Script/Engine.ProjectileMovementComponent|SetInitialSpeed _projectilemovement _travelspeed)
  (return))

(fn DisableProjectileMovement
  (bind _projectilemovement (Variables|Default|GetProjectileMovement))
  (Variables|/Script/Engine.ProjectileMovementComponent|SetMaxSpeed _projectilemovement 0.0)
  (Variables|/Script/Engine.ProjectileMovementComponent|SetInitialSpeed _projectilemovement 0.0)
  (Variables|/Script/Engine.MovementComponent|SetVelocity _projectilemovement "0, 0, 0")
  (return))