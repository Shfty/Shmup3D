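; Player homing missile in the Itano style that launches in a random direction within a forward cone and curves toward TargetEnemy.
; It rides a two-point spline whose endpoint tracks the target each tick, periodically dropping PlayerBullet collision capsules behind it.
; Enemy hits apply damage and trigger GameState hitstop.
; Impact, target loss or path timeout spawns an explosion, detaches the trail and hides the missile before delayed cleanup.
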(event Custom|ItanoDeath
  (if (Components|Activation|IsActive (Variables|Default|GetRootScene))
    (Game|SpawnActorfromClass (Variables|Default|GetExplosionActorClass) (Transformation|GetActorTransform) "AlwaysSpawn" 0 0)
    (Transformation|DetachFromComponent (Variables|Default|GetItanoTrail) "KeepWorld" "KeepWorld" "KeepWorld" true)
    (Actor|Tick|SetActorTickEnabled false)
    (Rendering|SetVisibility (Variables|Default|GetMaterialBillboard) false true)
    (Components|Activation|SetActive (Variables|Default|GetRootScene) false false)
    (Actor|SetLifeSpan 2.0)))

(event EventTick
  (params (DeltaSeconds :type Float%20%28single-precision%29))
  (bind _flightpath (Variables|Default|GetFlightPath))
  (bind _droppedcapsulelength (Variables|Default|GetDroppedCapsuleLength))
  (bind _targetenemy (Variables|Default|GetTargetEnemy))
  (if (and (Variables|Default|GetbIsOnPath) (Components|Activation|IsActive (Variables|Default|GetRootScene)))
    (Utilities|IsValid _targetenemy
      (:Is%20Valid
        (Spline|SetLocationatSplinePoint _flightpath (- (Spline|GetNumberOfSplinePoints _flightpath) 1) (Transformation|GetActorLocation _targetenemy) "World" true)
        (Utilities|FlowControl|Sequence
          (:then_0
            ;[1 1 1] Move along spline
            (bind _output_get (Variables|Default|SetTimeAlongSpline (+ DeltaSeconds (Variables|Default|GetTimeAlongSpline))))
            (Transformation|SetActorTransform (Spline|GetTransformatTime (Variables|Default|GetFlightPath) _output_get "World" false false) true))
          (:then_1
            ;[1 1 1] Spawn collision capsules along spline
            (bind _output_get_2 (Variables|Default|SetCapsuleDropAccumulator (+ (Variables|Default|GetCapsuleDropAccumulator) (* (Spline|GetSplineLength (Variables|Default|GetFlightPath)) (Utilities|Time|GetWorldDeltaSeconds)))))
            (if (>= _output_get_2 (Variables|Default|GetDroppedCapsuleLength))
              (bind _returnvalue (AddComponent|AddCapsuleComponent true (Transformation|GetActorTransform)))
              (Collision|SetCollisionProfileName _returnvalue "PlayerBullet" :!class /Script/Engine.PrimitiveComponent)
              (Components|Capsule|SetCapsuleSize _returnvalue (* _droppedcapsulelength 0.25) (* _droppedcapsulelength 0.5) true)
              (Transformation|AddRelativeRotation _returnvalue "-90.000000, 0, 0" false false)
              (Variables|Default|SetCapsuleDropAccumulator 0.0)))
          (:then_2
            (if (> (Variables|Default|GetTimeAlongSpline) 1.0)
              (CallFunction|ItanoDeath :!label _label)))))
      (:Is%20Not%20Valid
        (goto _label)))))

(event EventCollideBullet)

(event EventBeginPlay
  (bind _flightpath (Variables|Default|GetFlightPath))
  ;[1 1 1] Randomize facing inside cone
  (Transformation|SetActorRotation (Math|Rotator|MakeRotfromX (Class|KismetMathLibrary|RandomUnitVectorinCone (Transformation|GetActorForwardVector) (Math|Trig|DegreesToRadians 45.0))) true)
  ;[1 1 1] Setup flight path
  (Utilities|IsValid (Variables|Default|GetTargetEnemy)
    (:Is%20Valid
      (Spline|SetSplinePoints _flightpath (Utilities|Array|MakeArray (Transformation|GetActorLocation) (Transformation|GetActorLocation (Variables|Default|GetTargetEnemy))) "World" true)
      (Spline|SetTangentatSplinePoint _flightpath 0 (* (Transformation|GetActorForwardVector) 5e+03) "World" true)
      ;[1 1 1] Initialize capsule drop accumulator
      (Variables|Default|SetCapsuleDropAccumulator (Variables|Default|GetDroppedCapsuleLength)))
    (:Is%20Not%20Valid
      (Actor|DestroyActor))))

(event EventCollideEnemy
  (params (Enemy :type BP%20Enemy%20Object%20Reference))
  (bind _damagetype (Variables|Default|GetDamageType))
  (Game|Damage|ApplyDamage Enemy (Variables|Default|GetDamage) 0 0 _damagetype)
  (Default|EventHitstop (CallFunction|GetGameState) (Utilities|GetClassDefaults _damagetype))
  (CallFunction|ItanoDeath))

(event EventCollideWorld
  (CallFunction|ItanoDeath))

(fn ConstructionScript
  (|CallParentFunction))