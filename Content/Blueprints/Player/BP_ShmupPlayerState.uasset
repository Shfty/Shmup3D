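; Player state for a shoot-'em-up that holds health, Itano ammo, shock cannon charge, upgrade segments and the set of available weapons.
; BeginPlay fills health, ammo and charge to their maximums.
; Pickup-style functions add to each resource, clamped at its max except upgrade segments, with shock cannon recharge also playing a 2D sound.
; A weapon availability check matches the weapon's class against the available list.
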(event EventBeginPlay
  (Variables|Default|SetHealth (Variables|Default|GetMax%20Health))
  (Variables|Default|SetItanoAmmo (Variables|Default|GetMaxItanoAmmo))
  (Variables|Default|SetShockCannonCharge (Variables|Default|GetMaxShockCannonCharge)))

(event EventRechargeShockCannons
  (params (Amount :type Float%20%28single-precision%29))
  (Variables|Default|SetShockCannonCharge (Math|Float|Min(Float) (+ (Variables|Default|GetShockCannonCharge) Amount) (Variables|Default|GetMaxShockCannonCharge)))
  (Audio|PlaySound2D (Variables|Default|GetShockCannonRechargeSound)))

(fn ConstructionScript)

(fn GiveItanoAmmo
  (params (Amount :type Integer))
  (Variables|Default|SetItanoAmmo (Math|Integer|Min(Integer) (+ (Variables|Default|GetItanoAmmo) Amount) (Variables|Default|GetMaxItanoAmmo))))

(fn GiveHealth
  (params (Amount :type Integer))
  (Variables|Default|SetHealth (Math|Integer|Min(Integer) (+ (Variables|Default|GetHealth) Amount) (Variables|Default|GetMax%20Health))))

(fn GiveUpgradeSegments
  (params (Amount :type Integer))
  (CallFunction|AddIntbyReference (Variables|Default|GetUpgradeSegments) Amount))

(fn IsWeaponAvailable
  (params (Weapon :type S3D%20Player%20Weapon%20Object%20Reference))
  (return (Utilities|Array|ContainsItem (Variables|Default|GetAvailableWeapons) (Utilities|GetClass Weapon))))