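; Player bullet radar that shows the direction and proximity of the nearest bullet on a bubble around the actor.
; MatchStarted creates dynamic materials and enables Tick, which finds the closest of the GameState's BulletLocations.
; The dot's position averages recent samples and its size grows with proximity, while ring, dot and RadarLine blend from white to red.
; Enemy and pickup dot code is disconnected and never runs.
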(event EventMatchStarted
  (bind _ringmesh (Variables|Default|GetRingMesh))
  (bind _bulletdot (Variables|Default|GetBulletDot))
  (bind _bubblemesh (Variables|Default|GetBubbleMesh))
  (Utilities|FlowControl|Sequence
    (:then_0
      (bind _returnvalue (Rendering|Material|CreateDynamicMaterialInstance _bubblemesh 0 (Rendering|Material|GetMaterial _bubblemesh 0) :!class /Script/Engine.PrimitiveComponent))
      (Variables|Default|SetBubbleDynamicMaterial _returnvalue)
      (bind _outactors (Actor|GetAllActorsOfClass "/Script/Engine.DirectionalLight"))
      (Utilities|IsValid (Utilities|Array|Get(acopy) _outactors)
        (:Is%20Valid
          (Rendering|Material|SetVectorParameterValue _returnvalue "LightDirection" (Utilities|Struct|MakeLinearColor (.x (Math|Vector|GetForwardVector (Variables|/Script/Engine.Light|GetLightComponent (Utilities|Array|Get(acopy) _outactors)))) (.y (Math|Vector|GetForwardVector (Variables|/Script/Engine.Light|GetLightComponent (Utilities|Array|Get(acopy) _outactors)))) (.z (Math|Vector|GetForwardVector (Variables|/Script/Engine.Light|GetLightComponent (Utilities|Array|Get(acopy) _outactors)))) 1.0) :!class /Script/Engine.MaterialInstanceDynamic))))
    (:then_1
      (bind _returnvalue_2 (Rendering|Material|CreateDynamicMaterialInstance _ringmesh 0 (Rendering|Material|GetMaterial _ringmesh 0) :!class /Script/Engine.PrimitiveComponent))
      (Variables|Default|SetRingDynamicMaterial _returnvalue_2))
    (:then_2
      (bind _returnvalue_3 (Rendering|Material|CreateDynamicMaterialInstance _bulletdot 0 (Rendering|Material|GetMaterial _bulletdot 0) :!class /Script/Engine.PrimitiveComponent))
      (Variables|Default|SetDotDynamicMaterial _returnvalue_3))
    (:then_3
      (Actor|Tick|SetActorTickEnabled true))))

(event EventTick
  (params (DeltaSeconds :type Float%20%28single-precision%29))
  (Utilities|FlowControl|Sequence
    (:then_0
      (CallFunction|ProcessBulletLocations))
    (:then_1)
    (:then_2)
    (:then_3)))

(fn ConstructionScript
  (Transformation|SetRelativeScale3D (Variables|Default|GetBubbleMesh) (Math|Conversions|ToVector(Float) (Variables|Default|GetVisualizationRange)))
  (Effects|Components|ParticleSystem|SetFloatParameter (Variables|Default|GetRadarLine) "Thickness" 2.0))

(fn SetRadarDotPosition
  (params (RadarDot :type Static%20Mesh%20Component%20Object%20Reference) (TargetLocation :type Vector) (SphereSize :type Float%20%28single-precision%29))
  (bind _returnvalue (Transformation|GetActorLocation))
  (bind _range (Variables|Default|GetRange))
  (bind _visualizationrange (Variables|Default|GetVisualizationRange))
  (bind _returnvalue_2 (- TargetLocation _returnvalue))
  (bind _returnvalue_3 (Math|Vector|VectorLength _returnvalue_2))
  (bind _returnvalue_4 (Math|Vector|Normalize _returnvalue_2))
  (bind _returnvalue_5 (* _returnvalue_4 _visualizationrange))
  (bind _returnvalue_6 (/ _returnvalue_3 _range))
  (bind _returnvalue_7 (- 1.0 _returnvalue_6))
  (bind _returnvalue_8 (* _returnvalue_7 SphereSize))
  (if (<= _returnvalue_3 _range)
    (Transformation|SetRelativeTransform RadarDot (Math|Transform|MakeTransform _returnvalue_5 (Math|Rotator|MakeRotfromZ _returnvalue_5) (Math|Vector|MakeVector _returnvalue_8 _returnvalue_8 _returnvalue_8)) false true))
  (return))

(fn AddRadarDotsforActorType
  (params (ActorClass :type Actor%20Class%20Reference) (InstancedStaticMeshComponent :type Instanced%20Static%20Mesh%20Component%20Object%20Reference) (SphereSize :type Float%20%28single-precision%29)))

(fn ProcessBulletLocations
  (bind _radarline (Variables|Default|GetRadarLine))
  (bind _bulletdot (Variables|Default|GetBulletDot))
  (bind _radarline_2 (Variables|Default|GetRadarLine))
  (bind _visualizationrange (Variables|Default|GetVisualizationRange))
  (bind _closestbulletsmoothinglist (Variables|Default|GetClosestBulletSmoothingList))
  (bind _ringdynamicmaterial (Variables|Default|GetRingDynamicMaterial))
  (bind _relativelocation (Variables|/Script/Engine.SceneComponent|GetRelativeLocation _bulletdot))
  (for _array_element (Variables|/Script/Shmup3D.S3DGameState|GetBulletLocations (CallFunction|GetGameState))
    (if (or (< (Math|Vector|VectorLength (- _array_element (Transformation|GetActorLocation))) (LocalVariables|GetClosestBulletDistance)) (< (LocalVariables|GetClosestBulletDistance) 0.0))
      (LocalVariables|SetClosestBulletDistance (Math|Vector|VectorLength (- _array_element (Transformation|GetActorLocation))))
      (LocalVariables|SetClosestBulletLocation _array_element)))
  (if (>= (LocalVariables|GetClosestBulletDistance) 0.0)
    (Rendering|Material|SetVectorParameterValue _ringdynamicmaterial "EmissiveColor" (Math|Color|Lerp(LinearColor) "(R=2.000000,G=0.000000,B=0.000000,A=1.000000)" "(R=1.000000,G=1.000000,B=1.000000,A=1.000000)" (Math|Float|MapRangeClamped (LocalVariables|GetClosestBulletDistance) (* _visualizationrange 2.0) (* _visualizationrange 4.0) 0.0 1.0)) :!class /Script/Engine.MaterialInstanceDynamic)
    (Utilities|Array|Add _closestbulletsmoothinglist (LocalVariables|GetClosestBulletLocation))
    (if (> (Utilities|Array|Length _closestbulletsmoothinglist) 10)
      (Utilities|Array|RemoveIndex _closestbulletsmoothinglist))
    (CallFunction|SetRadarDotPosition (Variables|Default|GetBulletDot) (Math|Vector|GetVectorArrayAverage _closestbulletsmoothinglist) (Variables|Default|GetBulletSphereSize))
    (Effects|Components|ParticleSystem|SetColorParameter _radarline_2 "Color" (Math|Color|Lerp(LinearColor) "(R=2.000000,G=0.000000,B=0.000000,A=1.000000)" "(R=1.000000,G=1.000000,B=1.000000,A=1.000000)" (Math|Float|MapRangeClamped (LocalVariables|GetClosestBulletDistance) (* _visualizationrange 2.0) (* _visualizationrange 4.0) 0.0 1.0)))
    (Effects|Components|ParticleSystem|SetVectorParameter _radarline_2 "Source" (* _relativelocation 0.7))
    (Effects|Components|ParticleSystem|SetVectorParameter _radarline_2 "Target" (* _relativelocation 1.15))
    (else
      (Rendering|Material|SetVectorParameterValue _ringdynamicmaterial "EmissiveColor" "(R=1.000000,G=1.000000,B=1.000000,A=1.000000)" :!class /Script/Engine.MaterialInstanceDynamic)
      (Effects|Components|ParticleSystem|SetColorParameter _radarline "Color" "(R=1.000000,G=1.000000,B=1.000000,A=1.000000)")
      (Effects|Components|ParticleSystem|SetVectorParameter _radarline "Source" "0, 0, 0")
      (Effects|Components|ParticleSystem|SetVectorParameter _radarline "Target" "0, 0, 0"))))