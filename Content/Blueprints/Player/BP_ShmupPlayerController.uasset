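; Player controller for a shmup that handles mouse and axis camera rotation, game-only input, quitting and numpad slow/fast-motion debug keys.
; A timeline-driven quick turn applies per-update angle deltas to control rotation, allowing pitch input while blocking yaw-axis input.
; StrafeY sets turn direction, while StrafeX scales it to full or half, or disables it for positive X without Y.
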(event EventBeginPlay
  (Input|SetInputModeGameOnly))

(event Input|ActionEvents|InputActionQuitGame
  (params (Key :type Key%20Structure :default "AnyKey"))
  ;[1 1 1] Quit handler
  (:Pressed
    (Game|QuitGame 0 "Quit")))

(event Input|ActionEvents|InputActionQuickTurn
  (params (Key :type Key%20Structure :default "AnyKey"))
  ;[1 1 1] Quickturn handler
  (:Pressed
    (if (and (not (Audio|Components|Audio|IsPlaying (Variables|Default|GetQuickTurnTimeline))) (> (Variables|Default|GetQuickTurnMultiplier) 0.0))
      (Variables|Default|SetPrevQuickTurnAngle 0.0)
      (bind _quickturnangle (Timeline|QuickTurnTimeline PlayFromStart)
        (:Update
          (Pawn|SetControlRotation (Math|Rotator|CombineRotators (Pawn|GetControlRotation :!class /Script/Engine.Controller) (Math|Vector|RotatorfromAxisandAngle "0, 0,1.000000" (* (- _quickturnangle (Variables|Default|GetPrevQuickTurnAngle)) (Variables|Default|GetQuickTurnAngleSign) (Variables|Default|GetQuickTurnMultiplier)))))
          (Variables|Default|SetPrevQuickTurnAngle _quickturnangle))))))

(event Input|AxisEvents|InputAxisCameraYaw
  (params (AxisValue :type Float%20%28single-precision%29))
  ;[1 1 1] Camera rotation handlers
  (if (not (Audio|Components|Audio|IsPlaying (Variables|Default|GetQuickTurnTimeline)))
    (Class|PlayerController|AddYawInput (* AxisValue (Utilities|Time|GetWorldDeltaSeconds)))))

(event Input|AxisEvents|InputAxisStrafeX
  (params (AxisValue :type Float%20%28single-precision%29))
  (if (not (Audio|Components|Audio|IsPlaying (Variables|Default|GetQuickTurnTimeline)))
    (if (< AxisValue 0.0)
      (Variables|Default|SetQuickTurnMultiplier 1.0)
      (elif (and (> AxisValue 0.0) (== (Input|AxisValues|GetStrafeY) 0.0))
        (Variables|Default|SetQuickTurnMultiplier 0.0)
        (else
          (Variables|Default|SetQuickTurnMultiplier 0.5))))))

(event Input|AxisEvents|InputAxisCameraPitch
  (params (AxisValue :type Float%20%28single-precision%29))
  ;[1 1 1] Camera rotation handlers
  (Class|PlayerController|AddPitchInput (* AxisValue (Utilities|Time|GetWorldDeltaSeconds))))

(event Input|AxisEvents|InputAxisStrafeY
  (params (AxisValue :type Float%20%28single-precision%29))
  (if (and (not (Audio|Components|Audio|IsPlaying (Variables|Default|GetQuickTurnTimeline))) (!= AxisValue 0.0))
    (if (< AxisValue 0.0)
      (Variables|Default|SetQuickTurnAngleSign -1.0)
      (else
        (Variables|Default|SetQuickTurnAngleSign 1.0)))))

(event Input|MouseEvents|MouseX
  (params (AxisValue :type Float%20%28single-precision%29))
  ;[1 1 1] Camera rotation handlers
  (Class|PlayerController|AddYawInput AxisValue))

(event Input|MouseEvents|MouseY
  (params (AxisValue :type Float%20%28single-precision%29))
  ;[1 1 1] Camera rotation handlers
  (Class|PlayerController|AddPitchInput AxisValue))

(event Input|KeyboardEvents|NumPadSix
  (params (Key :type Key%20Structure :default "AnyKey"))
  ;[1 1 1] Debug VCR controls
  (:Pressed
    (Development|ExecuteConsoleCommand "slomo 5")))

(event Input|KeyboardEvents|NumPadFive
  (params (Key :type Key%20Structure :default "AnyKey"))
  ;[1 1 1] Debug VCR controls
  (:Pressed
    (Development|ExecuteConsoleCommand "slomo 1")))

(event Input|KeyboardEvents|NumPadFour
  (params (Key :type Key%20Structure :default "AnyKey"))
  ;[1 1 1] Debug VCR controls
  (:Pressed
    (Development|ExecuteConsoleCommand "slomo 0.1")))

(fn ConstructionScript)