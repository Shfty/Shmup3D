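; Player weapon that fires a pair of projectiles from two mirrored spheres, with a laser sight for each.
; The construction script spaces the spheres by TwinSeparation and copies the first one's material to the twin.
; Aim updates trace to the target, offset the endpoint along the control rotation's right vector, then rotate each sphere toward its point.
; Firing, only while active, spawns projectiles at both sphere transforms and plays a sound.
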(event EventUpdateAim
  (params (TargetPoint :type Vector))
  (bind _rootscene (Variables|Default|GetRootScene))
  (bind _sightcolor (Variables|Default|GetSightColor))
  (if (and (Components|Activation|IsActive _rootscene) (Rendering|IsVisible _rootscene))
    (bind (_outhit _returnvalue) (Collision|LineTraceByChannel (Transformation|GetActorLocation) TargetPoint "TraceTypeQuery1" false 0 "None"))
    (if _returnvalue
      (CallFunction|UpdateSpheres (.ImpactPoint (Collision|BreakHitResult _outhit)) _sightcolor)
      (else
        (CallFunction|UpdateSpheres (.TraceEnd (Collision|BreakHitResult _outhit)) _sightcolor)))))

(event EventFireProjectile
  (bind _twinsphere (Variables|Default|GetTwinSphere))
  (bind _sphere (Variables|Default|GetSphere))
  (bind _returnvalue (Transformation|GetWorldTransform _twinsphere))
  (bind _returnvalue_2 (Transformation|GetWorldTransform _sphere))
  (if (Components|Activation|IsActive (Variables|Default|GetRootScene))
    (Game|SpawnActorfromClass (Variables|Default|GetProjectileClass) (Math|Transform|MakeTransform (.location _returnvalue_2) (.rotation _returnvalue_2) "1,1,1") "AlwaysSpawn" 0 true 0)
    (Game|SpawnActorfromClass (Variables|Default|GetProjectileClass) (Math|Transform|MakeTransform (.location _returnvalue) (.rotation _returnvalue) "1,1,1") "AlwaysSpawn" 0 true 0)
    (Audio|PlaySoundatLocation (Variables|Default|GetFireSound) (Transformation|GetActorLocation))))

(fn ConstructionScript
  (bind _sphere (Variables|Default|GetSphere))
  (bind _twinsphere (Variables|Default|GetTwinSphere))
  (|CallParentFunction)
  (Transformation|SetRelativeLocation _sphere (Math|Vector|MakeVector 0.0 (Variables|Default|GetTwinSeparation) 0.0) false false)
  (Transformation|SetRelativeLocation _twinsphere (Math|Vector|MakeVector 0.0 (* (Variables|Default|GetTwinSeparation) -1.0) 0.0) false false)
  (Rendering|Material|SetMaterial _twinsphere 0 (Rendering|Material|GetMaterial _sphere 0)))

(fn UpdateSpheres
  (params (TraceEndpoint :type Vector) (LaserSightColor :type Linear%20Color%20Structure))
  (bind _returnvalue (Game|Player|GetPlayerPawn 0))
  (bind _twinseparation (Variables|Default|GetTwinSeparation))
  (bind _returnvalue_2 (Pawn|GetControlRotation _returnvalue :!class /Script/Engine.Pawn))
  (bind _returnvalue_3 (Math|Vector|GetRightVector _returnvalue_2))
  (bind _returnvalue_4 (* _returnvalue_3 _twinseparation))
  (CallFunction|UpdateSphereSingle (Variables|Default|GetSphere) (+ TraceEndpoint _returnvalue_4) LaserSightColor)
  (CallFunction|UpdateSphereSingle (Variables|Default|GetTwinSphere) (- TraceEndpoint _returnvalue_4) LaserSightColor)
  (return))

(fn UpdateSphereSingle
  (params (Sphere :type Scene%20Component%20Object%20Reference) (TraceEndpoint :type Vector) (LaserSightColor :type Linear%20Color%20Structure))
  (bind _returnvalue (Transformation|GetWorldLocation Sphere))
  (CallFunction|DrawLaserSight _returnvalue TraceEndpoint LaserSightColor 2.5e+02 5.0 5.0)
  (Transformation|SetWorldRotation Sphere (Math|Rotator|MakeRotfromX (Math|Vector|Normalize (- TraceEndpoint _returnvalue))) false false)
  (return))