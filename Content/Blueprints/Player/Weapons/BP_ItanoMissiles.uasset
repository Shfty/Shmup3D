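; Player lock-on missile swarm weapon with twin launchers placed symmetrically by the construction script.
; While fire is held, a looping timer locks shuffled enemies from the play volume, spending PlayerState ammo per lock until the limit or ammo runs out.
; Locked enemies requeue, allowing stacked locks and icons on one target.
; Release spawns one homing missile per lock in a single loop, alternating launchers via FlipFlop and clearing icons.
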(event Custom|AddTargetEnemy
  (bind _candidateenemies (Variables|Default|GetCandidateEnemies))
  (bind _item (Utilities|Array|Get(acopy) _candidateenemies))
  (bind _asbp_enemy (Utilities|Casting|CastToBP_Enemy _item))
  (if (Math|Boolean|ANDBoolean (> (Utilities|Array|Length _candidateenemies) 0) (< (Utilities|Array|Length (Variables|Default|GetTargetedEnemies)) (Variables|Default|GetTargetLimit)) (> (Variables|/Game/Blueprints/Player/BP_ShmupPlayerState.BP_ShmupPlayerState_C|GetItanoAmmo (CallFunction|GetPlayerState)) 0)) :!label _label
    (Utilities|IsValid _item
      (:Is%20Valid
        (Audio|PlaySound2D "/Game/Sounds/SoundCues/Effects/MissileSwarmLock_Cue.MissileSwarmLock_Cue")
        (Default|AddLockIcon (.AsBP%20Itano%20Lock%20on%20Widget%20UMG (Utilities|Casting|CastToBP_ItanoLockOnWidgetUMG (UserInterface|GetUserWidgetObject (Variables|/Game/Blueprints/Enemies/BP_Enemy.BP_Enemy_C|GetItanoLockOnWidget _asbp_enemy)))))
        (Utilities|Array|Add (Variables|Default|GetTargetedEnemies) _asbp_enemy)
        (Utilities|Array|Add _candidateenemies _asbp_enemy)
        (Utilities|Array|RemoveIndex _candidateenemies)
        (CallFunction|SubtractIntbyReference (Variables|/Game/Blueprints/Player/BP_ShmupPlayerState.BP_ShmupPlayerState_C|GetItanoAmmo (CallFunction|GetPlayerState)) (Variables|Default|GetAmmoUsePerMissile)))
      (:Is%20Not%20Valid
        (Utilities|Array|RemoveIndex _candidateenemies)
        (goto _label)))
    (else
      (Utilities|Time|ClearandInvalidateTimerbyHandle (stale EventBeginFire _output_get))
      (Utilities|Array|Clear (Variables|Default|GetCandidateEnemies)))))

(event EventUpdateAim
  (params (TargetPoint :type Vector)))

(event EventBeginFire
  (bind _candidateenemies (Variables|Default|GetCandidateEnemies))
  (bind _candidateenemies_2 (Variables|Default|GetCandidateEnemies))
  (bind _item (Utilities|Array|Get(acopy) _candidateenemies))
  (bind _asbp_enemy (Utilities|Casting|CastToBP_Enemy _item))
  (if (and (not (Utilities|Time|IsTimerActivebyHandle (Variables|Default|GetFiringTimer))) (Components|Activation|IsActive (Variables|Default|GetRootScene)))
    (Utilities|Array|AppendArray _candidateenemies_2 (Variables|/Script/Shmup3D.S3DGameState|GetEnemiesInPlayVolume (CallFunction|GetGameState)))
    (Utilities|Array|Shuffle _candidateenemies_2)
    (bind _returnvalue (Utilities|Time|SetTimerbyEvent (delegate Custom|AddTargetEnemy) (Variables|Default|GetTargetingRate) true))
    (bind _output_get (Variables|Default|SetTargetingTimer _returnvalue))
    (if (Math|Boolean|ANDBoolean (> (Utilities|Array|Length _candidateenemies) 0) (< (Utilities|Array|Length (Variables|Default|GetTargetedEnemies)) (Variables|Default|GetTargetLimit)) (> (Variables|/Game/Blueprints/Player/BP_ShmupPlayerState.BP_ShmupPlayerState_C|GetItanoAmmo (CallFunction|GetPlayerState)) 0)) :!label _label
      (Utilities|IsValid _item
        (:Is%20Valid
          (Audio|PlaySound2D "/Game/Sounds/SoundCues/Effects/MissileSwarmLock_Cue.MissileSwarmLock_Cue")
          (Default|AddLockIcon (.AsBP%20Itano%20Lock%20on%20Widget%20UMG (Utilities|Casting|CastToBP_ItanoLockOnWidgetUMG (UserInterface|GetUserWidgetObject (Variables|/Game/Blueprints/Enemies/BP_Enemy.BP_Enemy_C|GetItanoLockOnWidget _asbp_enemy)))))
          (Utilities|Array|Add (Variables|Default|GetTargetedEnemies) _asbp_enemy)
          (Utilities|Array|Add _candidateenemies _asbp_enemy)
          (Utilities|Array|RemoveIndex _candidateenemies)
          (CallFunction|SubtractIntbyReference (Variables|/Game/Blueprints/Player/BP_ShmupPlayerState.BP_ShmupPlayerState_C|GetItanoAmmo (CallFunction|GetPlayerState)) (Variables|Default|GetAmmoUsePerMissile)))
        (:Is%20Not%20Valid
          (Utilities|Array|RemoveIndex _candidateenemies)
          (goto _label)))
      (else
        (Utilities|Time|ClearandInvalidateTimerbyHandle _output_get)
        (Utilities|Array|Clear (Variables|Default|GetCandidateEnemies))))))

(event EventEndFire
  (bind _twinsphere (Variables|Default|GetTwinSphere))
  (bind _targetedenemies (Variables|Default|GetTargetedEnemies))
  (bind _targetedenemies_2 (Variables|Default|GetTargetedEnemies))
  (bind _sphere (Variables|Default|GetSphere))
  (bind _returnvalue (Utilities|Array|Length _targetedenemies_2))
  (bind _item (Utilities|Array|Get(acopy) _targetedenemies))
  (bind _returnvalue_2 (Transformation|GetWorldTransform _twinsphere))
  (bind _returnvalue_3 (Transformation|GetWorldTransform _sphere))
  (bind _returnvalue_4 (> _returnvalue 0))
  (if (Components|Activation|IsActive (Variables|Default|GetRootScene))
    (Utilities|Array|Clear (Variables|Default|GetCandidateEnemies))
    (Utilities|Time|ClearandInvalidateTimerbyHandle (Variables|Default|GetTargetingTimer))
    (if _returnvalue_4
      (while _returnvalue_4
        (if (Components|Activation|IsActive (Variables|Default|GetRootScene))
          (if (> (Utilities|Array|Length (Variables|Default|GetTargetedEnemies)) 0)
            (Utilities|IsValid _item
              (:Is%20Valid
                (Utilities|FlowControl|FlipFlop
                  (:A
                    (Game|SpawnActorfromClass "/Game/Blueprints/Player/Projectiles/BP_ItanoMissile.BP_ItanoMissile_C" (Math|Transform|MakeTransform (.location _returnvalue_3) (.rotation _returnvalue_3) "1,1,1") "AlwaysSpawn" 0 _item true _item))
                  (:B
                    (Game|SpawnActorfromClass "/Game/Blueprints/Player/Projectiles/BP_ItanoMissile.BP_ItanoMissile_C" (Math|Transform|MakeTransform (.location _returnvalue_2) (.rotation _returnvalue_2) "1,1,1") "AlwaysSpawn" 0 0 true _item)))
                (Default|ClearLockIcons (.AsBP%20Itano%20Lock%20on%20Widget%20UMG (Utilities|Casting|CastToBP_ItanoLockOnWidgetUMG (UserInterface|GetUserWidgetObject (Variables|/Game/Blueprints/Enemies/BP_Enemy.BP_Enemy_C|GetItanoLockOnWidget _item)))))
                (Utilities|Array|RemoveIndex (Variables|Default|GetTargetedEnemies)))
              (:Is%20Not%20Valid
                (Utilities|Array|RemoveItem _targetedenemies _item)))
            (else
              (Utilities|Time|ClearandInvalidateTimerbyHandle (Variables|Default|GetFiringTimer))))))
      (Audio|PlaySound2D "/Game/Sounds/SoundCues/Effects/MissileSwarmFire_Cue.MissileSwarmFire_Cue"))))

(fn ConstructionScript
  (bind _sphere (Variables|Default|GetSphere))
  (bind _twinsphere (Variables|Default|GetTwinSphere))
  (|CallParentFunction)
  ;[1 1 1] Configure twin mesh
  (Transformation|SetRelativeLocation _sphere (Math|Vector|MakeVector 0.0 (Variables|Default|GetTwinSeparation) 0.0) false false)
  (Transformation|SetRelativeLocation _twinsphere (Math|Vector|MakeVector 0.0 (* (Variables|Default|GetTwinSeparation) -1.0) 0.0) false false)
  (Rendering|Material|SetMaterial _twinsphere 0 (Rendering|Material|GetMaterial _sphere 0)))