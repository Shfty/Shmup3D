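; BP_ShockCannons is a twin-cannon player weapon that fires projectiles from two mirrored spheres, spending ShockCannonCharge from the player state per shot.
; While active and visible, UpdateAim line-traces to the target point, rotating both spheres toward the hit or trace end and drawing laser sights.
; FireProjectile alternates spawns between the spheres via FlipFlop, relative to the play volume, and plays a fire sound.
; The construction script spaces the spheres by TwinSeparation and matches their materials.
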(event EventUpdateAim
  (params (TargetPoint :type Vector))
  (bind _rootscene (Variables|Default|GetRootScene))
  (bind _sightcolor (Variables|Default|GetSightColor))
  (if (and (Components|Activation|IsActive _rootscene) (Rendering|IsVisible _rootscene))
    (bind (_outhit _returnvalue) (Collision|LineTraceByChannel (Transformation|GetActorLocation) TargetPoint "TraceTypeQuery1" false 0 "None"))
    (if _returnvalue
      (CallFunction|UpdateSpheres (.ImpactPoint (Collision|BreakHitResult _outhit)) _sightcolor)
      (else
        (CallFunction|UpdateSpheres (.TraceEnd (Collision|BreakHitResult _outhit)) _sightcolor)))))

(event EventFireProjectile
  (bind _playerstate (CallFunction|GetPlayerState))
  (bind _chargepershot (Variables|Stats|GetChargePerShot))
  (bind _twinsphere (Variables|Default|GetTwinSphere))
  (bind _sphere (Variables|Default|GetSphere))
  (bind _returnvalue (Transformation|GetWorldTransform _twinsphere))
  (bind _returnvalue_2 (Transformation|GetWorldTransform _sphere))
  (bind _shockcannoncharge (Variables|/Game/Blueprints/Player/BP_ShmupPlayerState.BP_ShmupPlayerState_C|GetShockCannonCharge _playerstate))
  (if (and (Components|Activation|IsActive (Variables|Default|GetRootScene)) (>= _shockcannoncharge _chargepershot))
    (CallFunction|SubtractFloatbyReference _shockcannoncharge _chargepershot)
    (Utilities|FlowControl|FlipFlop
      (:A
        (Game|SpawnActorfromClass (Variables|Default|GetProjectileClass) (Math|Transform|MakeTransform (.location _returnvalue_2) (.rotation _returnvalue_2) "2.000000,2.000000,1") "AlwaysSpawn" 0 true 0))
      (:B
        (Game|SpawnActorfromClass (Variables|Default|GetProjectileClass) (Math|Transform|MakeTransform (.location _returnvalue) (.rotation _returnvalue) "2.000000,2.000000,1") "AlwaysSpawn" 0 true 0)))
    (Audio|PlaySoundatLocation (Variables|Default|GetFireSound) (Transformation|GetActorLocation))))

(fn ConstructionScript
  (bind _sphere (Variables|Default|GetSphere))
  (bind _twinsphere (Variables|Default|GetTwinSphere))
  (|CallParentFunction)
  (Transformation|SetRelativeLocation _sphere (Math|Vector|MakeVector 0.0 (Variables|Stats|GetTwinSeparation) 0.0) false false)
  (Transformation|SetRelativeLocation _twinsphere (Math|Vector|MakeVector 0.0 (* (Variables|Stats|GetTwinSeparation) -1.0) 0.0) false false)
  (Rendering|Material|SetMaterial _twinsphere 0 (Rendering|Material|GetMaterial _sphere 0)))

(fn UpdateSpheres
  (params (TraceEndpoint :type Vector) (LaserSightColor :type Linear%20Color%20Structure))
  (CallFunction|UpdateSphereSingle (Variables|Default|GetSphere) TraceEndpoint LaserSightColor)
  (CallFunction|UpdateSphereSingle (Variables|Default|GetTwinSphere) TraceEndpoint LaserSightColor))

(fn UpdateSphereSingle
  (params (Sphere :type Scene%20Component%20Object%20Reference) (TraceEndpoint :type Vector) (LaserSightColor :type Linear%20Color%20Structure))
  (bind _returnvalue (Transformation|GetWorldLocation Sphere))
  (CallFunction|DrawLaserSight _returnvalue TraceEndpoint LaserSightColor 5e+02 25.0 5.0)
  (Transformation|SetWorldRotation Sphere (Math|Rotator|MakeRotfromX (Math|Vector|Normalize (- TraceEndpoint _returnvalue))) false false)
  (return))