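; Player weapon Blueprint that auto-fires projectiles while held and aims with an enemy-locking laser sight.
; BeginFire starts a looping timer that fires while active, calling the parent's projectile logic only below a world-wide projectile cap.
; UpdateAim rotates the weapon toward the target, then line-traces to set TargetEnemy and draw the sight with debug-circle reticles.
; A sphere-trace multi-lock sight exists but is never called.
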(event Custom|Event%20Refire
  (if (Variables|State|GetbIsActive)
    (CallFunction|FireProjectile)))

(event EventEndFire
  (Utilities|Time|ClearandInvalidateTimerbyHandle (Variables|State|GetFireTimer)))

(event EventUpdateAim
  (params (TargetPoint :type Vector))
  (bind _returnvalue (Transformation|GetActorLocation))
  (bind _rootscene (Variables|Default|GetRootScene))
  (bind _returnvalue_2 (- TargetPoint _returnvalue))
  (bind _returnvalue_3 (Math|Vector|Normalize _returnvalue_2))
  (bind _returnvalue_4 (Math|Vector|CrossProduct _returnvalue_3 "0, 0,1.000000"))
  (bind _returnvalue_5 (Math|Vector|Normalize _returnvalue_4))
  ;[1 1 1] Comment
  (Transformation|SetActorRotation (Math|Rotator|MakeRotfromX _returnvalue_3))
  ;[1 1 1] Calculate laser sight YZ axes
  (if (and (Components|Activation|IsActive _rootscene) (Rendering|IsVisible _rootscene))
    (Variables|Default|SetLaserSightY _returnvalue_5)
    (Variables|Default|SetLaserSightZ (Math|Vector|Normalize (Math|Vector|CrossProduct _returnvalue_5 _returnvalue_3)))
    (CallFunction|DrawSingleLockLaserSight TargetPoint)))

(event EventFireProjectile
  (bind _outactors (Actor|GetAllActorsOfClass (Variables|Default|GetProjectileClass)))
  (if (< (Utilities|Array|Length _outactors) (Variables|Default|GetMaxProjectileCount))
    (|CallParentFunction)))

(event EventBeginFire
  (bind _returnvalue (Utilities|Time|SetTimerbyEvent (delegate Custom|Event%20Refire) (Variables|Stats|GetFireRate) true))
  (Variables|State|SetFireTimer _returnvalue)
  (if (Variables|State|GetbIsActive)
    (CallFunction|FireProjectile)))

(fn ConstructionScript
  (|CallParentFunction))

(fn DrawMultiLockLaserSight
  (params (TargetPoint :type Vector))
  (bind _aimtraceradius (Variables|Default|GetAimTraceRadius))
  (bind _lasersighty (Variables|Default|GetLaserSightY))
  (bind _lasersightz (Variables|Default|GetLaserSightZ))
  ;[1 1 1] Trace aim line inside play bounds and draw
  (bind _outhit (Collision|LineTraceForObjects (Transformation|GetActorLocation) TargetPoint (Utilities|Array|MakeArray "ObjectTypeQuery8") false 0 "None"))
  (CallFunction|DrawLaserSight (.TraceStart (Collision|BreakHitResult _outhit)) (.ImpactPoint (Collision|BreakHitResult _outhit)) (Variables|Default|GetSightColor) 1e+03 _aimtraceradius 1e+01)
  (Rendering|Debug|DrawDebugCircle (.ImpactPoint (Collision|BreakHitResult _outhit)) _aimtraceradius 32 "(R=1.000000,G=1.000000,B=1.000000,A=1.000000)" 0.0 1e+01 _lasersighty _lasersightz true)
  (Rendering|Debug|DrawDebugCircle (.ImpactPoint (Collision|BreakHitResult _outhit)) 2e+01 32 "(R=1.000000,G=1.000000,B=1.000000,A=1.000000)" 0.0 5.0 _lasersighty _lasersightz true)
  ;[1 1 1] Sphere trace for enemies and draw lock on reticles
  (Variables|Default|SetTargetEnemy 0)
  (bind _outhits (Collision|MultiSphereTraceForObjects (.TraceStart (Collision|BreakHitResult _outhit)) (.ImpactPoint (Collision|BreakHitResult _outhit)) (Variables|Default|GetAimTraceRadius) (Utilities|Array|MakeArray "ObjectTypeQuery9") false 0 "None"))
  (Utilities|Array|Clear (Variables|Default|GetIgnoredTraceActors))
  (for _array_element _outhits
    (if (not (Utilities|Array|ContainsItem (Variables|Default|GetIgnoredTraceActors) (.HitActor (Collision|BreakHitResult _array_element))))
      (Utilities|FlowControl|Sequence
        (:then_0
          (Rendering|Debug|DrawDebugCircle (+ (.TraceStart (Collision|BreakHitResult _array_element)) (* (- (.TraceEnd (Collision|BreakHitResult _array_element)) (.TraceStart (Collision|BreakHitResult _array_element))) (.Time (Collision|BreakHitResult _array_element)))) (Variables|Default|GetAimTraceRadius) 32 "(R=10.000000,G=0.000000,B=0.000000,A=1.000000)" 0.0 1e+01 (Variables|Default|GetLaserSightY) (Variables|Default|GetLaserSightZ) true)
          (Utilities|Array|Add (Variables|Default|GetIgnoredTraceActors) (.HitActor (Collision|BreakHitResult _array_element))))
        (:then_1
          (Utilities|IsValid (Variables|Default|GetTargetEnemy)
            (:Is%20Valid
              _)
            (:Is%20Not%20Valid
              (bind _ass3denemy (Utilities|Casting|CastToS3DEnemy (.HitActor (Collision|BreakHitResult _array_element)))
                (:then
                  (Variables|Default|SetTargetEnemy _ass3denemy))
                (:CastFailed
                  _)))))))
    (return))
  (return))

(fn DrawSingleLockLaserSight
  (params (TargetPoint :type Vector))
  (bind _returnvalue (Transformation|GetActorLocation))
  (bind _aimtraceradius (Variables|Default|GetAimTraceRadius))
  (bind _lasersighty (Variables|Default|GetLaserSightY))
  (bind _lasersightz (Variables|Default|GetLaserSightZ))
  (bind _aimtraceradius_2 (Variables|Default|GetAimTraceRadius))
  (bind _lasersighty_2 (Variables|Default|GetLaserSightY))
  (bind _lasersightz_2 (Variables|Default|GetLaserSightZ))
  (bind _aimtraceradius_3 (Variables|Default|GetAimTraceRadius))
  (bind _lasersighty_3 (Variables|Default|GetLaserSightY))
  (bind _lasersightz_3 (Variables|Default|GetLaserSightZ))
  ;[1 1 1] Trace aim line inside play bounds and draw
  (bind (_outhit _returnvalue_2) (Collision|LineTraceForObjects _returnvalue TargetPoint (Utilities|Array|MakeArray "ObjectTypeQuery9") false 0 "None"))
  (if _returnvalue_2
    (CallFunction|DrawLaserSight (.TraceStart (Collision|BreakHitResult _outhit)) (.ImpactPoint (Collision|BreakHitResult _outhit)) (Variables|Default|GetSightColor) 1e+03 _aimtraceradius_2 1e+01)
    (Rendering|Debug|DrawDebugCircle (.ImpactPoint (Collision|BreakHitResult _outhit)) _aimtraceradius_2 32 "(R=1.000000,G=0.000000,B=0.000000,A=1.000000)" 0.0 1e+01 _lasersighty_2 _lasersightz_2 true)
    (Rendering|Debug|DrawDebugCircle (.ImpactPoint (Collision|BreakHitResult _outhit)) 2e+01 32 "(R=1.000000,G=0.000000,B=0.000000,A=1.000000)" 0.0 5.0 _lasersighty_2 _lasersightz_2 true)
    (bind _ass3denemy (Utilities|Casting|CastToS3DEnemy (.HitActor (Collision|BreakHitResult _outhit))))
    (Variables|Default|SetTargetEnemy _ass3denemy)
    ;[1 1 1] Trace aim line inside play bounds and draw
    (bind _outhit_2 (Collision|LineTraceForObjects (.ImpactPoint (Collision|BreakHitResult _outhit)) TargetPoint (Utilities|Array|MakeArray "ObjectTypeQuery8") false 0 "None"))
    (CallFunction|DrawLaserSight (.TraceStart (Collision|BreakHitResult _outhit_2)) (.ImpactPoint (Collision|BreakHitResult _outhit_2)) "(R=1.000000,G=0.000000,B=0.000000,A=1.000000)" 1e+03 _aimtraceradius_3 1e+01)
    (Rendering|Debug|DrawDebugCircle (.ImpactPoint (Collision|BreakHitResult _outhit_2)) _aimtraceradius_3 32 "(R=1.000000,G=1.000000,B=1.000000,A=1.000000)" 0.0 1e+01 _lasersighty_3 _lasersightz_3 true)
    (Rendering|Debug|DrawDebugCircle (.ImpactPoint (Collision|BreakHitResult _outhit_2)) 2e+01 32 "(R=1.000000,G=1.000000,B=1.000000,A=1.000000)" 0.0 5.0 _lasersighty_3 _lasersightz_3 true)
    (else
      ;[1 1 1] Trace aim line inside play bounds and draw
      (bind _outhit_3 (Collision|LineTraceForObjects _returnvalue TargetPoint (Utilities|Array|MakeArray "ObjectTypeQuery8") false 0 "None"))
      (CallFunction|DrawLaserSight (.TraceStart (Collision|BreakHitResult _outhit_3)) (.ImpactPoint (Collision|BreakHitResult _outhit_3)) "(R=0.000000,G=1.000000,B=0.782499,A=1.000000)" 1e+03 _aimtraceradius 1e+01)
      (Rendering|Debug|DrawDebugCircle (.ImpactPoint (Collision|BreakHitResult _outhit_3)) _aimtraceradius 32 "(R=1.000000,G=1.000000,B=1.000000,A=1.000000)" 0.0 1e+01 _lasersighty _lasersightz true)
      (Rendering|Debug|DrawDebugCircle (.ImpactPoint (Collision|BreakHitResult _outhit_3)) 2e+01 32 "(R=1.000000,G=1.000000,B=1.000000,A=1.000000)" 0.0 5.0 _lasersighty _lasersightz true)
      (Variables|Default|SetTargetEnemy 0))))