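; Player ship pawn for a shmup, handling free 3D flight, weapons, damage and timed respawn.
; Boost starts a barrel roll with a shield and enlarged damage sphere, suppressing the active weapon and turning incoming hits into Shock Cannon charge.
; Tick banks the mesh from velocity and aims the active weapon along the camera view.
; Health lives in the player state; hits grant flashing invincibility, ramming hurts both sides and crushing kills.
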(event EventTick
  (params (DeltaSeconds :type Float%20%28single-precision%29))
  (Utilities|FlowControl|Sequence
    (:then_1
      ;[1 1 1] Flash ship if invincible
      (if (Class|KismetSystemLibrary|TimerExistsHandle (Variables|State|Lifecycle|GetHitInvincibilityTimer))
        (Rendering|ToggleVisibility (Variables|Default|GetShipMesh) true) ; Flash ship mesh every frame
      ))
    (:then_2
      ;[1 1 1] Add forward movement if no direction is held during boost
      (if (and (Variables|State|GetbIsBoosting) (Math|Vector|Equal(Vector) (Math|Vector|MakeVector (Input|AxisValues|GetStrafeX) (Input|AxisValues|GetStrafeY) (Input|AxisValues|GetStrafeZ)) "0, 0, 0" 0.0))
        (Movement|Accelerate (Math|Vector|GetForwardVector (Pawn|GetControlRotation :!class /Script/Engine.Pawn)) 1.0)))
    (:then_3
      (Movement|UpdateShipOrientation))
    (:then_4
      (Weapons|UpdateWeapons))
    (:then_5
      (Variables|Default|SetPreviousVelocity (Variables|/Script/Engine.MovementComponent|GetVelocity (Variables|Default|GetFloatingPawnMovement))))))

(event OnComponentBeginOverlap(CrushCollider)
  (params (OverlappedComponent :type Primitive%20Component%20Object%20Reference) (OtherActor :type Actor%20Object%20Reference) (OtherComp :type Primitive%20Component%20Object%20Reference) (OtherBodyIndex :type Integer) (bFromSweep :type Boolean) (SweepResult :type Hit%20Result%20Structure%20%28by%20ref%29))
  (bind _playerstate (CallFunction|GetPlayerState))
  ;[1 1 1] Crush death handler
  (Utilities|IsValid _playerstate
    (:Is%20Valid
      (if (> (Variables|/Game/Blueprints/Player/BP_ShmupPlayerState.BP_ShmupPlayerState_C|GetHealth _playerstate) 0)
        (Variables|/Game/Blueprints/Player/BP_ShmupPlayerState.BP_ShmupPlayerState_C|SetHealth (CallFunction|GetPlayerState) 0)
        (CallFunction|EventPlayerDeath)))))

(event Custom|Event%20RespawnExpired
  ;[1 1 1] Death/Respawn handler
  (Audio|PlaySoundatLocation (Variables|Default|GetRespawnSound) (Transformation|GetActorLocation))
  (Effects|SpawnEmitterAttached (Variables|Stats|Effects|GetRespawnParticleSytem) (Variables|Default|GetRootSphere) "None" "0, 0, 0" "0, 0, 0" "SnapToTarget")
  (Utilities|Time|SetTimerbyEvent (delegate Custom|Event%20ActivateShip) 0.8))

(event Custom|Event%20ActivateShip
  ;[1 1 1] Death/Respawn handler
  (State|SetShipActive true)
  (Variables|/Game/Blueprints/Player/BP_ShmupPlayerState.BP_ShmupPlayerState_C|SetHealth (CallFunction|GetPlayerState) (Variables|Stats|Lifecycle|GetMaxHealth))
  (CallFunction|EventHitInvincibility))

(event Custom|Event%20PlayerDeath
  ;[1 1 1] Death/Respawn handler
  (Audio|PlaySoundatLocation (Variables|Default|GetDeathSound) (Transformation|GetActorLocation))
  (Effects|SpawnEmitterAttached (Variables|Stats|Effects|GetDeathParticleSystem) (Variables|Default|GetRootSphere) "None" "0, 0, 0" "0, 0, 0" "SnapToTarget")
  (State|SetShipActive false)
  (bind _returnvalue (Utilities|Time|SetTimerbyEvent (delegate Custom|Event%20RespawnExpired) (Variables|Stats|Lifecycle|GetRespawnDuration)))
  (Variables|State|Lifecycle|SetRespawnTimer _returnvalue))

(event Custom|Event%20HitInvincibilityExpired
  ;[1 1 1] Hit invincibility handler
  (Utilities|Time|ClearandInvalidateTimerbyHandle (Variables|State|Lifecycle|GetHitInvincibilityTimer))
  (Rendering|SetVisibility (Variables|Default|GetShipMesh) true true))

(event Custom|Event%20HitInvincibility
  ;[1 1 1] Hit invincibility handler
  (bind _returnvalue (Utilities|Time|SetTimerbyEvent (delegate Custom|Event%20HitInvincibilityExpired) (Variables|Stats|Lifecycle|GetHitInvincibilityDuration)))
  (Variables|State|Lifecycle|SetHitInvincibilityTimer _returnvalue))

(event Game|Damage|EventAnyDamage
  (params (Damage :type Float%20%28single-precision%29) (DamageType :type Damage%20Type%20Object%20Reference) (InstigatedBy :type Controller%20Object%20Reference) (DamageCauser :type Actor%20Object%20Reference))
  (bind _playerstate (CallFunction|GetPlayerState))
  ;[1 1 1] Damage handler
  (if (and (not (Utilities|Time|IsTimerActivebyHandle (Variables|State|Lifecycle|GetHitInvincibilityTimer))) (> (Variables|/Game/Blueprints/Player/BP_ShmupPlayerState.BP_ShmupPlayerState_C|GetHealth (CallFunction|GetPlayerState)) 0))
    (if (not (Variables|Default|GetbIsInvulnerable))
      (Audio|PlaySoundatLocation (Variables|Default|GetDamageSound) (Transformation|GetActorLocation))
      (bind _output_get (Variables|/Game/Blueprints/Player/BP_ShmupPlayerState.BP_ShmupPlayerState_C|SetHealth _playerstate (Math|Integer|Max(Integer) (- (Variables|/Game/Blueprints/Player/BP_ShmupPlayerState.BP_ShmupPlayerState_C|GetHealth _playerstate) (Math|Float|Round Damage)))))
      (if (== _output_get 0)
        (CallFunction|EventPlayerDeath)
        (else
          (CallFunction|EventHitInvincibility)))
      (else
        (Class|S3DPlayerState|RechargeShockCannons (CallFunction|GetPlayerState) (Variables|/Script/Shmup3D.S3DDamageType|GetShockCannonChargeOnBulletHit (.AsS3DDamage%20Type (Utilities|Casting|CastToS3DDamageType DamageType))))))))

(event Collision|EventActorBeginOverlap
  (params (OtherActor :type Actor%20Object%20Reference))
  ;[1 1 1] Enemy ram handler
  (if (and (not (Utilities|Time|IsTimerActivebyHandle (Variables|State|Lifecycle|GetHitInvincibilityTimer))) (Utilities|ClassIsChildOf (Utilities|GetClass OtherActor) "/Game/Blueprints/Enemies/BP_Enemy.BP_Enemy_C"))
    (Game|Damage|ApplyDamage OtherActor (Variables|Stats|GetRamDamage) 0 0)
    (Game|Damage|ApplyDamage self 1.0 0 0 "/Game/Blueprints/DamageTypes/BP_EnemyRamDamage.BP_EnemyRamDamage_C")))

(event Custom|Event%20BoostEnd
  (bind _activeweapon (Variables|Default|GetActiveWeapon))
  ;[1 1 1] Boost input handler
  (Variables|State|SetbIsBoosting false)
  (CallFunction|SetMovementParameters (Variables|Stats|Movement|GetMoveSpeed) (Variables|Stats|Movement|GetAcceleration) (Variables|Stats|Movement|GetDeceleration))
  (Audio|Components|Audio|Stop (Variables|Default|GetBoostLoopAudio))
  (Components|Activation|SetActive (Variables|Default|GetBoostTrail) false true)
  (Utilities|IsValid _activeweapon
    (:Is%20Valid
      (Components|Activation|SetActive (Variables|/Game/Blueprints/Player/BP_PlayerWeapon.BP_PlayerWeapon_C|GetRootScene _activeweapon) true false)
      (if (Variables|State|GetbFirePressed)
        (Default|BeginFire (Variables|Default|GetActiveWeapon))))))

(event Input|ActionEvents|InputActionFire
  (params (Key :type Key%20Structure :default "AnyKey"))
  (bind _activeweapon (Variables|Default|GetActiveWeapon))
  ;[1 1 1] Fire input handler
  (:Pressed
    (Variables|State|SetbFirePressed true)
    (Variables|Default|SetCachedOrientation (Pawn|GetControlRotation :!class /Script/Engine.Pawn))
    (Utilities|IsValid _activeweapon
      (:Is%20Valid
        (Default|BeginFire _activeweapon))))
  (:Released
    (Variables|State|SetbFirePressed false)
    (Utilities|IsValid _activeweapon
      (:Is%20Valid
        (Default|EndFire _activeweapon)))))

(event Input|ActionEvents|InputActionWeaponSlot1
  (params (Key :type Key%20Structure :default "AnyKey"))
  ;[1 1 1] Weapon keys
  (:Pressed
    (Weapons|TrySwitchWeapon)))

(event Input|ActionEvents|InputActionWeaponSlot2
  (params (Key :type Key%20Structure :default "AnyKey"))
  ;[1 1 1] Weapon keys
  (:Pressed
    (Weapons|TrySwitchWeapon 1)))

(event Input|ActionEvents|InputActionWeaponSlot3
  (params (Key :type Key%20Structure :default "AnyKey"))
  ;[1 1 1] Weapon keys
  (:Pressed
    (Weapons|TrySwitchWeapon 2)))

(event Input|ActionEvents|InputActionNextWeapon
  (params (Key :type Key%20Structure :default "AnyKey"))
  ;[1 1 1] Next/Prev Weapon Keys
  (:Pressed
    (bind _weaponindex (CallFunction|FindRelativeWeaponIndex 1))
    (Weapons|TrySwitchWeapon _weaponindex)))

(event Input|ActionEvents|InputActionPrevWeapon
  (params (Key :type Key%20Structure :default "AnyKey"))
  ;[1 1 1] Next/Prev Weapon Keys
  (:Pressed
    (bind _weaponindex (CallFunction|FindRelativeWeaponIndex -1))
    (Weapons|TrySwitchWeapon _weaponindex)))

(event Input|ActionEvents|InputActionItanoMissiles
  (params (Key :type Key%20Structure :default "AnyKey"))
  (bind _itanomissiles (Variables|Default|GetItanoMissiles))
  (bind _childactor (Variables|/Script/Engine.ChildActorComponent|GetChildActor _itanomissiles))
  (bind _asbp_itano_missiles (Utilities|Casting|CastToBP_ItanoMissiles _childactor))
  ;[1 1 1] Itano missile handler
  (:Pressed
    (Default|BeginFire _asbp_itano_missiles))
  (:Released
    (Default|EndFire _asbp_itano_missiles)))

(event Input|ActionEvents|InputActionBoost
  (params (Key :type Key%20Structure :default "AnyKey"))
  (bind _activeweapon (Variables|Default|GetActiveWeapon))
  (bind _barrelrolltimeline (Variables|Default|GetBarrelRollTimeline))
  (bind _boosttrail (Variables|Default|GetBoostTrail))
  (bind _returnvalue (Audio|Components|Audio|IsPlaying _barrelrolltimeline))
  (bind _rootscene (Variables|/Game/Blueprints/Player/BP_PlayerWeapon.BP_PlayerWeapon_C|GetRootScene _activeweapon))
  (bind _returnvalue_2 (not _returnvalue))
  ;[1 1 1] Boost input handler
  (:Pressed
    (Variables|State|SetbBoostPressed true)
    (if (and (not (Variables|State|GetbIsBoosting)) _returnvalue_2)
      (Components|Timeline|PlayfromStart (Variables|Default|GetBarrelRollTimeline))
      (Audio|PlaySoundatLocation (Variables|Default|GetBoostSound) (Transformation|GetActorLocation))
      (Variables|State|SetbIsBoosting true)
      (Variables|Default|SetbIsInvulnerable true)
      (Rendering|SetVisibility (Variables|Default|GetShieldMesh) true true)
      (CallFunction|SetBoostDamageSphereActive true)
      (Utilities|FlowControl|Sequence
        (:then_0
          (Components|Timeline|PlayfromStart (Variables|Default|GetBoostSpeedTimeline)))
        (:then_1
          (Components|Activation|SetActive _boosttrail true false)
          (Utilities|IsValid _activeweapon
            (:Is%20Valid
              (Components|Activation|SetActive _rootscene false false))
            (:Is%20Not%20Valid
              _))
          (Transformation|SetRelativeRotation (Variables|Default|GetShipMesh) (Math|Conversions|RotationFromXVector (Pawn|Components|PawnMovement|GetLastInputVector (Variables|Default|GetFloatingPawnMovement))) false false)))))
  (:Released
    (Variables|State|SetbBoostPressed false)
    (if _returnvalue_2
      (Variables|State|SetbIsBoosting false)
      (CallFunction|SetMovementParameters (Variables|Stats|Movement|GetMoveSpeed) (Variables|Stats|Movement|GetAcceleration) (Variables|Stats|Movement|GetDeceleration))
      (Audio|Components|Audio|Stop (Variables|Default|GetBoostLoopAudio))
      (Components|Activation|SetActive _boosttrail false true)
      (Utilities|IsValid _activeweapon
        (:Is%20Valid
          (Components|Activation|SetActive _rootscene true false)
          (if (Variables|State|GetbFirePressed)
            (Default|BeginFire (Variables|Default|GetActiveWeapon))))))))

(event Input|AxisEvents|InputAxisStrafeX
  (params (AxisValue :type Float%20%28single-precision%29))
  (bind _returnvalue (Pawn|GetControlRotation :!class /Script/Engine.Pawn))
  (bind _returnvalue_2 (Math|Vector|GetForwardVector _returnvalue))
  ;[1 1 1] Strafe input handler
  (Movement|Accelerate (Math|Vector|Normalize (Math|Vector|MakeVector (.x _returnvalue_2) (.y _returnvalue_2) 0.0)) AxisValue))

(event Input|AxisEvents|InputAxisStrafeY
  (params (AxisValue :type Float%20%28single-precision%29))
  ;[1 1 1] Strafe input handler
  (Movement|Accelerate (Math|Vector|GetRightVector (Pawn|GetControlRotation :!class /Script/Engine.Pawn)) AxisValue))

(event Input|AxisEvents|InputAxisStrafeZ
  (params (AxisValue :type Float%20%28single-precision%29))
  ;[1 1 1] Strafe input handler
  (Movement|Accelerate "0, 0,1.000000" AxisValue))

(event EventBeginPlay
  (Rendering|SetVisibility (Variables|Default|GetShieldMesh) false true))

(event EventMatchStarted
  (Utilities|FlowControl|Sequence
    (:then_0)
    (:then_1
      ;[1 1 1] Setup weapons
      (bind _output_get (Variables|Default|SetWeapons (Utilities|Array|MakeArray (.AsBP%20Player%20Weapon (Utilities|Casting|CastToBP_PlayerWeapon (Variables|/Script/Engine.ChildActorComponent|GetChildActor (Variables|Default|GetBasicWeapon)))) (.AsBP%20Player%20Weapon (Utilities|Casting|CastToBP_PlayerWeapon (Variables|/Script/Engine.ChildActorComponent|GetChildActor (Variables|Default|GetTwinMissiles)))) (.AsBP%20Player%20Weapon (Utilities|Casting|CastToBP_PlayerWeapon (Variables|/Script/Engine.ChildActorComponent|GetChildActor (Variables|Default|GetShockCannons)))))))
      (Variables|Default|SetActiveWeapon (Utilities|Array|Get(acopy) _output_get))
      (Default|CallWeaponSwitched 0))
    (:then_2
      (Actor|Tick|SetActorTickEnabled true :!pinned true) ; Enable tick
    )))

(fn ConstructionScript
  (bind _floatingpawnmovement (Variables|Default|GetFloatingPawnMovement))
  (Variables|/Script/Engine.FloatingPawnMovement|SetMaxSpeed _floatingpawnmovement (Variables|Stats|Movement|GetMoveSpeed))
  (Variables|/Script/Engine.FloatingPawnMovement|SetAcceleration _floatingpawnmovement (Variables|Stats|Movement|GetAcceleration))
  (Variables|/Script/Engine.FloatingPawnMovement|SetDeceleration _floatingpawnmovement (Variables|Stats|Movement|GetDeceleration))
  (Variables|Default|SetCachedDamageSphereRadius (Variables|/Script/Engine.SphereComponent|GetSphereRadius (Variables|Default|GetDamageCollider))))

(fn Accelerate
  (params (Vector :type Vector) (Input :type Float%20%28single-precision%29))
  (Class|PawnMovementComponent|AddInputVector (Variables|Default|GetFloatingPawnMovement) (* Vector Input) false)
  (return))

(fn GetCameraAttachTransform
  (bind _cameraattachpoint (Variables|Default|GetCameraAttachPoint))
  (return (Transformation|GetWorldLocation _cameraattachpoint) (Transformation|GetWorldRotation _cameraattachpoint)))

(fn SetShipActive
  (params (New%20Active :type Boolean))
  (bind _returnvalue (Actor|GetComponentsbyTag "/Script/Engine.PrimitiveComponent" "Collision"))
  (bind _floatingpawnmovement (Variables|Default|GetFloatingPawnMovement))
  (if New%20Active
    (for _array_element _returnvalue
      (Collision|SetCollisionEnabled _array_element "QueryOnly"))
    (else
      (for _array_element_2 _returnvalue
        (Collision|SetCollisionEnabled _array_element_2 "NoCollision"))))
  (Rendering|SetVisibility (Variables|Default|GetShipMesh) New%20Active true)
  (Variables|/Script/Engine.MovementComponent|SetVelocity _floatingpawnmovement "0, 0, 0")
  (Components|Activation|SetActive _floatingpawnmovement New%20Active false)
  (return))

(fn TrySwitchWeapon
  (params (WeaponIndex :type Integer))
  (bind _weapons (Variables|Default|GetWeapons))
  (bind _item (Utilities|Array|Get(acopy) _weapons WeaponIndex))
  (if (and (< WeaponIndex (Utilities|Array|Length _weapons)) (Default|IsWeaponAvailable (.AsBP%20Shmup%20Player%20State (Utilities|Casting|CastToBP_ShmupPlayerState (Variables|Default|GetPlayerState))) _item))
    (Utilities|IsValid (Variables|Default|GetActiveWeapon)
      (:Is%20Valid
        (Default|EndFire (Variables|Default|GetActiveWeapon))
        (Components|Activation|SetActive (Variables|/Game/Blueprints/Player/BP_PlayerWeapon.BP_PlayerWeapon_C|GetRootScene (Variables|Default|GetActiveWeapon)) false false))
      (:Is%20Not%20Valid
        _))
    (bind _output_get (Variables|Default|SetActiveWeapon _item))
    (if (Weapons|CanFire)
      (Components|Activation|SetActive (Variables|/Game/Blueprints/Player/BP_PlayerWeapon.BP_PlayerWeapon_C|GetRootScene _output_get) true false)
      (if (Variables|State|GetbFirePressed)
        (Default|BeginFire _output_get)))
    (Default|CallWeaponSwitched WeaponIndex)))

(fn CanFire
  (return (not (Variables|State|GetbIsBoosting))))

(fn TrackPlayVolume
  (bind _returnvalue (Game|GetPlayerController 0))
  (bind _returnvalue_2 (Transformation|GetActorLocation))
  (bind _playvolume (CallFunction|GetPlayVolume))
  (bind _rootsphere (Variables|Default|GetRootSphere))
  (bind _returnvalue_3 (Transformation|GetActorLocation _playvolume))
  (bind _returnvalue_4 (Transformation|GetActorTransform _playvolume))
  (bind _returnvalue_5 (- _returnvalue_3 _returnvalue_2))
  (Utilities|IsValid _playvolume
    (:Is%20Valid
      (Transformation|SetWorldRotation _rootsphere (Transformation|GetActorRotation _playvolume) false false)
      (Class|SceneComponent|AddLocalTransform _rootsphere (Class|KismetMathLibrary|ConvertTransformtoRelative (Variables|State|BoundsTracking|GetLastBoundsTransform) _returnvalue_4) true true)
      (Transformation|AddWorldOffset (Variables|Default|GetRootSphere) (- _returnvalue_5 (Math|Vector|RotateVector _returnvalue_5 (.Rotation (Math|Transform|BreakTransform (Class|KismetMathLibrary|ConvertTransformtoRelative (Variables|State|BoundsTracking|GetLastBoundsTransform) _returnvalue_4))))) true true)
      (Pawn|SetControlRotation _returnvalue (Math|Rotator|CombineRotators (Pawn|GetControlRotation _returnvalue :!class /Script/Engine.Controller) (.Rotation (Math|Transform|BreakTransform (Class|KismetMathLibrary|ConvertTransformtoRelative (Variables|State|BoundsTracking|GetLastBoundsTransform) _returnvalue_4)))))
      (Variables|State|BoundsTracking|SetLastBoundsTransform _returnvalue_4)
      (return))
    (:Is%20Not%20Valid
      (return))))

(fn UpdateShipOrientation
  (bind _shipmesh (Variables|Default|GetShipMesh))
  (bind _previousvelocity (Variables|Default|GetPreviousVelocity))
  (bind _floatingpawnmovement (Variables|Default|GetFloatingPawnMovement))
  (bind _returnvalue (Math|Vector|Normalize _previousvelocity))
  (bind _velocity (Variables|/Script/Engine.MovementComponent|GetVelocity _floatingpawnmovement))
  (bind _returnvalue_2 (Math|Vector|CrossProduct _velocity "0, 0,-1.000000"))
  (bind _returnvalue_3 (Math|Vector|Normalize _velocity))
  (bind _returnvalue_4 (Math|Vector|CrossProduct _returnvalue_3 _returnvalue))
  (bind _returnvalue_5 (* (.z _returnvalue_4) -3.6e+02))
  (bind _returnvalue_6 (Math|Vector|RotateVectorAroundAxis _returnvalue_2 _returnvalue_5 _returnvalue_3))
  (Utilities|FlowControl|Sequence
    (:then_0
      ;[1 1 1] Determine state for rotation calculation
      (if (not (Class|KismetSystemLibrary|TimerExistsHandle (Variables|State|Lifecycle|GetRespawnTimer))) ; Are we currently dead?
        (if (or (Variables|State|GetbIsBoosting) (Audio|Components|Audio|IsPlaying (Variables|Default|GetBarrelRollTimeline)))
          ;[1 1 1] Boost orientation
          (Variables|State|SetTargetShipRotation (Math|Rotator|MakeRotationfromAxes (Math|Vector|RotateVectorAroundAxis _returnvalue_3 _returnvalue_5 "0, 0,1.000000") _returnvalue_6 (Math|Vector|RotateVectorAroundAxis (* (Math|Vector|CrossProduct _returnvalue_3 (Math|Vector|Normalize _returnvalue_6)) -1.0) _returnvalue_5 "0, 0,1.000000")))
          (else
            ;[1 1 1] Roll ship mesh based on velocity
            (Variables|State|SetTargetShipRotation (Math|Rotator|CombineRotators (Math|Rotator|MakeRotator (* (Math|Vector|DotProduct (Math|Vector|ClampVectorSize (Variables|/Script/Engine.MovementComponent|GetVelocity (Variables|Default|GetFloatingPawnMovement)) 0.0 (Variables|Stats|Movement|GetMoveSpeed)) (Math|Vector|GetRightVector (Variables|Default|GetShipMesh))) 0.025) 0.0 0.0) (Transformation|GetActorRotation)))))))
    (:then_1
      ;[1 1 1] Interpolate ship rotation
      (Transformation|SetRelativeRotation _shipmesh (Math|Interpolation|RInterpTo (Variables|/Script/Engine.SceneComponent|GetRelativeRotation _shipmesh) (Variables|State|GetTargetShipRotation) (Utilities|Time|GetWorldDeltaSeconds) (Variables|Stats|Movement|GetShipRotationInterpSpeed)) false false))
    (:then_2
      (return))))

(fn UpdateWeapons
  (bind _activeweapon (Variables|Default|GetActiveWeapon))
  (LocalVariables|SetWeaponOrientation (Pawn|GetControlRotation :!class /Script/Engine.Pawn))
  ;[1 1 1] Update active weapon aim
  (Utilities|IsValid _activeweapon
    (:Is%20Valid
      (Default|UpdateAim _activeweapon (+ (Camera|GetCameraLocation (Game|GetPlayerCameraManager 0)) (* (Math|Vector|GetForwardVector (LocalVariables|GetWeaponOrientation)) (Variables|Stats|GetAimTraceLength)))))
    (:Is%20Not%20Valid
      _))
  (return))

(fn GetPlayerState
  (bind _asbp_shmup_player_state (Utilities|Casting|CastToBP_ShmupPlayerState (Variables|Default|GetPlayerState))
    (:then
      (return _asbp_shmup_player_state))
    (:CastFailed
      (return 0))))

(fn SetMovementParameters
  (params (MaxSpeed :type Float%20%28single-precision%29) (Acceleration :type Float%20%28single-precision%29) (Deceleration :type Float%20%28single-precision%29))
  (bind _floatingpawnmovement (Variables|Default|GetFloatingPawnMovement))
  (Variables|/Script/Engine.FloatingPawnMovement|SetMaxSpeed _floatingpawnmovement MaxSpeed)
  (Variables|/Script/Engine.FloatingPawnMovement|SetAcceleration _floatingpawnmovement Acceleration)
  (Variables|/Script/Engine.FloatingPawnMovement|SetDeceleration _floatingpawnmovement Deceleration)
  (return))

(fn SetBoostDamageSphereActive
  (params (Active :type Boolean))
  (if Active
    (Components|Sphere|SetSphereRadius (Variables|Default|GetDamageCollider) (* (Variables|Default|GetCachedDamageSphereRadius) (Variables|Default|GetBoostDamageSphereRadiusMultiplier)) true)
    (else
      (Components|Sphere|SetSphereRadius (Variables|Default|GetDamageCollider) (Variables|Default|GetCachedDamageSphereRadius) true)))
  (return))

(fn FindRelativeWeaponIndex
  (params (RelativeIndex :type Integer))
  (bind _weapons (Variables|Default|GetWeapons))
  (bind _activeweapon (Variables|Default|GetActiveWeapon))
  (bind _returnvalue (Utilities|Array|FindItem _weapons _activeweapon))
  (bind _returnvalue_2 (Utilities|Array|Length _weapons))
  (bind _returnvalue_3 (- _returnvalue_2 1))
  (bind _returnvalue_4 (+ _returnvalue RelativeIndex))
  (if (> _returnvalue_4 _returnvalue_3)
    (return 0)
    (elif (< _returnvalue_4 0)
      (return _returnvalue_3)
      (else
        (return _returnvalue_4)))))