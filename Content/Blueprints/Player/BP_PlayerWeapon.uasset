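; BP_PlayerWeapon is a player weapon Blueprint that spawns projectiles and leaves BeginFire, EndFire and UpdateAim as empty hooks.
; FireProjectile runs only while the root scene is active and the player state reports this weapon as available.
; It spawns the configured projectile class at the weapon's transform, passing the target enemy and a move-relative-to-play-volume flag, then plays the fire sound at the weapon's location.
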(event Custom|BeginFire)

(event Custom|EndFire)

(fn ConstructionScript)

(fn FireProjectile
  (if (and (Components|Activation|IsActive (Variables|Default|GetRootScene)) (Default|IsWeaponAvailable (CallFunction|GetPlayerState) self))
    (Game|SpawnActorfromClass (Variables|Stats|GetProjectileClass) (Transformation|GetActorTransform) "AlwaysSpawn" 0 true (Variables|State|GetTargetEnemy))
    (Audio|PlaySoundatLocation (Variables|Stats|GetFireSound) (Transformation|GetActorLocation))))

(fn UpdateAim
  (params (TargetPoint :type Vector)))