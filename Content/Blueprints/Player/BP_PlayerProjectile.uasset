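; Base player projectile that damages enemies and destroys itself on impact.
; It can attach to the play volume on spawn to move relative to it.
; Hitbox overlaps split into enemy hits, which apply damage and trigger game-state hitstop from the damage type, or world hits.
; Both, plus any damage received (treated as a bullet collision), spawn a death particle effect and destroy the actor.
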(event OnComponentBeginOverlap(DamageHitbox)
  (params (OverlappedComponent :type Primitive%20Component%20Object%20Reference) (OtherActor :type Actor%20Object%20Reference) (OtherComp :type Primitive%20Component%20Object%20Reference) (OtherBodyIndex :type Integer) (bFromSweep :type Boolean) (SweepResult :type Hit%20Result%20Structure%20%28by%20ref%29))
  (bind _asbp_enemy (Utilities|Casting|CastToBP_Enemy OtherActor)
    (:then
      (CallFunction|CollideEnemy _asbp_enemy))
    (:CastFailed
      (CallFunction|CollideWorld))))

(event Custom|CollideEnemy
  (params (Enemy :type BP%20Enemy%20Object%20Reference))
  (bind _damagetype (Variables|Default|GetDamageType))
  (Game|Damage|ApplyDamage Enemy (Variables|Default|GetDamage) 0 0 _damagetype)
  (Default|EventHitstop (CallFunction|GetGameState) (Utilities|GetClassDefaults _damagetype))
  (CallFunction|SpawnDeathEffectandDestroySelf))

(event Custom|CollideBullet
  (CallFunction|SpawnDeathEffectandDestroySelf))

(event Custom|CollideWorld
  (CallFunction|SpawnDeathEffectandDestroySelf))

(event Game|Damage|EventAnyDamage
  (params (Damage :type Float%20%28single-precision%29) (DamageType :type Damage%20Type%20Object%20Reference) (InstigatedBy :type Controller%20Object%20Reference) (DamageCauser :type Actor%20Object%20Reference))
  (CallFunction|CollideBullet))

(event EventBeginPlay
  (if (Variables|Default|GetbMoveRelativeToPlayVolume)
    (Transformation|AttachActorToActor (CallFunction|GetPlayVolume) "None" "KeepWorld" "KeepWorld" "KeepWorld" false)))

(fn ConstructionScript)

(fn SpawnDeathEffectandDestroySelf
  (bind _rootscene (Variables|Default|GetRootScene))
  (Utilities|IsValid _rootscene
    (:Is%20Valid
      (Effects|SpawnEmitteratLocation (Variables|Default|GetDeathParticleSystem) (Transformation|GetWorldLocation _rootscene))
      (Actor|DestroyActor)
      (return))
    (:Is%20Not%20Valid
      (return))))