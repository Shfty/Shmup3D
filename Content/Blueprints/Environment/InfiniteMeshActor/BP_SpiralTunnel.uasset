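; BP_SpiralTunnel is an environment actor that scrolls a tunnel mesh continuously, speeding up once the match starts.
; On MatchStarted, a timeline drives ScrollRate along an acceleration curve.
; Each tick adds ScrollRate scaled by delta time to MeshScroll, then calls the parent Tick, leaving the mesh update and construction to the parent class.
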(event EventTick
  (params (DeltaSeconds :type Float%20%28single-precision%29))
  (Variables|Default|SetMeshScroll (+ (Variables|Default|GetMeshScroll) (* (Variables|Default|GetScrollRate) DeltaSeconds)))
  (|CallParentFunction DeltaSeconds))

(event EventMatchStarted
  (bind _scrollrate (Timeline|AccelerationTimeline Play)
    (:Update
      (Variables|Default|SetScrollRate _scrollrate))))

(fn ConstructionScript
  (|CallParentFunction))