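; BP_InfiniteMeshActor fakes an endlessly scrolling stack of static meshes by recycling components along Z.
; Construction stacks meshes from MeshSequence by bounds height under OffsetScene, centered on the actor.
; Tick moves them by the change in MeshScroll and resets any passing the top to zero with the next sequence mesh.
; BufferMeshReplacement queues one-time swaps by sequence index, and BeginPlay queues a spiral hole mesh at index zero.
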(event EventTick
  (params (DeltaSeconds :type Float%20%28single-precision%29))
  (bind _meshsequence (Variables|Stats|GetMeshSequence))
  (bind _meshreplacementindices (Variables|Default|GetMeshReplacementIndices))
  (for _array_element (Variables|State|GetStaticMeshComponents)
    (Transformation|AddRelativeLocation _array_element (Math|Vector|MakeVector 0.0 0.0 (- (Variables|State|GetMeshScroll) (Variables|State|GetPrevMeshScroll))) false true)
    (if (> (.z (Variables|/Script/Engine.SceneComponent|GetRelativeLocation _array_element)) (Variables|State|GetTotalMeshHeight))
      (Transformation|SetRelativeLocation _array_element (Math|Vector|MakeVector 0.0 0.0 0.0) false true)
      (bind _result (Math|Integer|IncrementInt (Variables|State|GetMeshSequenceIndex))
        (:%20%20
          (if (!= (Utilities|Array|FindItem _meshreplacementindices (Math|Integer|%(Integer) _result (Utilities|Array|Length _meshsequence))) -1)
            (Components|StaticMesh|SetStaticMesh _array_element (Utilities|Array|Get(acopy) (Variables|Default|GetMeshReplacements) (Utilities|Array|FindItem _meshreplacementindices (Math|Integer|%(Integer) _result (Utilities|Array|Length _meshsequence)))))
            (Utilities|Array|RemoveIndex _meshreplacementindices (Utilities|Array|FindItem _meshreplacementindices (Math|Integer|%(Integer) _result (Utilities|Array|Length _meshsequence))))
            (Utilities|Array|RemoveIndex (Variables|Default|GetMeshReplacements) (Utilities|Array|FindItem _meshreplacementindices (Math|Integer|%(Integer) _result (Utilities|Array|Length _meshsequence))))
            (else
              (Components|StaticMesh|SetStaticMesh _array_element (Utilities|Array|Get(acopy) _meshsequence (Math|Integer|%(Integer) _result (Utilities|Array|Length _meshsequence))))))))))
  (Variables|State|SetPrevMeshScroll (Variables|State|GetMeshScroll)))

(event EventBeginPlay
  (CallFunction|BufferMeshReplacement 0 "/Game/Meshes/SM_InfiniteMeshSpiralHole.SM_InfiniteMeshSpiralHole"))

(fn ConstructionScript
  (bind _totalmeshheight (Variables|State|GetTotalMeshHeight))
  (Utilities|FlowControl|Sequence
    (:then_0
      ;[1 1 1] Create mesh instances
      (for _index (range 0 (- (Variables|Stats|GetNumMeshes) 1))
        (bind _returnvalue (AddComponent|AddStaticMeshComponent true (Math|Transform|MakeTransform (Math|Vector|MakeVector 0.0 0.0 _totalmeshheight) "0, 0, 0" "1,1,1")))
        (CallFunction|AddFloatbyReference _totalmeshheight (* (.Z (Math|Vector|BreakVector (.boxextent (StaticMesh|GetBounds (Utilities|Array|Get(acopy) (Variables|Stats|GetMeshSequence) (Math|Integer|%(Integer) _index (Utilities|Array|Length (Variables|Stats|GetMeshSequence)))))))) 2.0))
        (Components|StaticMesh|SetStaticMesh _returnvalue (Utilities|Array|Get(acopy) (Variables|Stats|GetMeshSequence) (Math|Integer|%(Integer) _index (Utilities|Array|Length (Variables|Stats|GetMeshSequence)))))
        (Transformation|AttachComponentToComponent _returnvalue (Variables|Default|GetOffsetScene) "None" "KeepRelative" "KeepRelative" "KeepRelative" false)
        (Utilities|Array|Add (Variables|State|GetStaticMeshComponents) _returnvalue)
        (Math|Integer|IncrementInt (Variables|State|GetMeshSequenceIndex))))
    (:then_1
      ;[1 1 1] Setup mesh offset
      (Transformation|SetRelativeLocation (Variables|Default|GetOffsetScene) (Math|Vector|MakeVector 0.0 0.0 (* (Variables|State|GetTotalMeshHeight) -0.5)) false false))))

(fn BufferMeshReplacement
  (params (IndexToReplace :type Integer) (StaticMesh :type Static%20Mesh%20Object%20Reference))
  (Utilities|Array|Add (Variables|Default|GetMeshReplacementIndices) IndexToReplace)
  (Utilities|Array|Add (Variables|Default|GetMeshReplacements) StaticMesh))