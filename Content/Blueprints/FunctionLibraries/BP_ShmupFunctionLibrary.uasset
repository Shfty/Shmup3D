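; Blueprint function library of shared helpers for the shmup game.
; Typed getters cast the game mode, state, instance, player pawn, player state and play volume (a stopgap until BP_PlayVolume moves to C++).
; By-reference int and float add/subtract helpers write back and return the result, alongside a relative-transform helper.
; DrawLaserSight draws a debug line with evenly spaced rings that brighten toward the end point.
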(fn GetGameMode
  (return (.AsBP%20Shmup%20Game%20Mode (Utilities|Casting|CastToBP_ShmupGameMode (Game|GetGameMode)))))

(fn GetGameState
  (return (.AsBP%20Shmup%20Game%20State (Utilities|Casting|CastToBP_ShmupGameState (Game|GetGameState)))))

(fn GetPlayVolume
  (bind _asbp_play_volume (Utilities|Casting|CastToBP_PlayVolume (Variables|/Script/Shmup3D.S3DGameState|GetPlayVolume (GameplayFramework|GetGameState))) ; TODO: Remove when BP_PlayVolume is ported to C++
    (:then
      (return _asbp_play_volume))
    (:CastFailed
      (return 0))))

(fn GetRelativeTransform
  (params (A :type Transform) (B :type Transform))
  (return (Math|Transform|ComposeTransforms A (Math|Transform|InvertTransform B))))

(fn DrawLaserSight
  (params (Start :type Vector) (End :type Vector) (Color :type Linear%20Color%20Structure) (SubdivisionLength :type Float%20%28single-precision%29) (RingSize :type Float%20%28single-precision%29) (RingThickness :type Float%20%28single-precision%29))
  (bind _returnvalue (- Start End))
  (bind _returnvalue_2 (- End Start))
  (bind _returnvalue_3 (Math|Vector|VectorLength _returnvalue))
  (bind _returnvalue_4 (Math|Vector|Normalize _returnvalue_2))
  (bind _returnvalue_5 (/ _returnvalue_3 SubdivisionLength))
  (bind _returnvalue_6 (Math|Vector|CrossProduct _returnvalue_4 "0, 0,1.000000"))
  (bind _returnvalue_7 (Math|Vector|Normalize _returnvalue_6))
  (bind _returnvalue_8 (Math|Float|Floor _returnvalue_5))
  (bind _returnvalue_9 (Math|Vector|CrossProduct _returnvalue_7 _returnvalue_4))
  (bind _returnvalue_10 (Math|Vector|Normalize _returnvalue_9))
  (for _index (range 1 _returnvalue_8)
    (Rendering|Debug|DrawDebugCircle 0 (+ Start (* _returnvalue_4 (* _index SubdivisionLength))) RingSize 32 (* Color (Math|Float|Clamp(Float) (/ (Math|Conversions|ToFloat(Integer) _index) (Math|Conversions|ToFloat(Integer) _returnvalue_8)) 0.0)) 0.0 RingThickness _returnvalue_7 _returnvalue_10)
    (Rendering|Debug|DrawDebugCircle 0 (+ Start (* _returnvalue_4 (* _index SubdivisionLength))) 5.0 32 (* Color (Math|Float|Clamp(Float) (/ (Math|Conversions|ToFloat(Integer) _index) (Math|Conversions|ToFloat(Integer) _returnvalue_8)) 0.0)) 0.0 5.0 _returnvalue_7 _returnvalue_10))
  (Rendering|Debug|DrawDebugLine 0 Start End Color 0.0)
  (return))

(fn GetPlayerState
  (params (PlayerIndex :type Integer))
  (bind _asbp_shmup_player_state (Utilities|Casting|CastToBP_ShmupPlayerState (Variables|/Script/Engine.Pawn|GetPlayerState (GameplayFramework|GetPlayerPawn PlayerIndex)))
    (:then
      (return _asbp_shmup_player_state))
    (:CastFailed
      (return 0))))

(fn GetPlayerPawn
  (params (PlayerIndex :type Integer))
  (bind _asbp_shmup_player_pawn (Utilities|Casting|CastToBP_ShmupPlayerPawn (Game|Player|GetPlayerPawn 0 PlayerIndex))
    (:then
      (return _asbp_shmup_player_pawn))
    (:CastFailed
      (return 0))))

(fn AddIntbyReference
  (params (LHS :type Integer%20%28by%20ref%29) (RHS :type Integer))
  (bind _returnvalue (+ LHS RHS))
  (|SetBy-RefVar LHS _returnvalue)
  (return _returnvalue))

(fn SubtractIntbyReference
  (params (LHS :type Integer%20%28by%20ref%29) (RHS :type Integer))
  (bind _returnvalue (- LHS RHS))
  (|SetBy-RefVar LHS _returnvalue)
  (return _returnvalue))

(fn SubtractFloatbyReference
  (params (LHS :type Float%20%28single-precision%29%20%28by%20ref%29) (RHS :type Float%20%28single-precision%29))
  (bind _returnvalue (- LHS RHS))
  (|SetBy-RefVar LHS _returnvalue)
  (return _returnvalue))

(fn GetOwningPlayerPawn
  (params (Widget :type User%20Widget%20Object%20Reference))
  (bind _asbp_shmup_player_pawn (Utilities|Casting|CastToBP_ShmupPlayerPawn (Class|UserWidget|GetOwningPlayerPawn Widget))
    (:then
      (return _asbp_shmup_player_pawn))
    (:CastFailed
      (return 0))))

(fn GetGameInstance
  (bind _ass3dgame_instance (Utilities|Casting|CastToS3DGameInstance (Game|GetGameInstance))
    (:then
      (return _ass3dgame_instance))
    (:CastFailed
      (return 0))))

(fn AddFloatbyReference
  (params (LHS :type Float%20%28single-precision%29%20%28by%20ref%29) (RHS :type Float%20%28single-precision%29))
  (bind _returnvalue (+ LHS RHS))
  (|SetBy-RefVar LHS _returnvalue)
  (return _returnvalue))