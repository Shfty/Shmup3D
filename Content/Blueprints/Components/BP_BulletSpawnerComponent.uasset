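; Actor component that fires enemy bullets from its owner at a fixed rate.
; On initialization it gets a bullet particle emitter from the game state, configured with the enemy bullet template, material, space, lifetime, size and collision size.
; A looping timer, started only for a positive spawn rate, has that emitter spawn a bullet at the set velocity whenever the component is active.
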(event Custom|Initialize
  (bind _bulletspawnrate (Variables|Bullets|Parameters|GetBulletSpawnRate))
  (bind _returnvalue (Class|S3DGameState|GetBulletParticleComponent (CallFunction|GetGameState) "/Game/ParticleSystems/Bullets/PS_EnemyBullets.PS_EnemyBullets" (Variables|Bullets|ParticleSystem|GetBulletMaterial) (Variables|Bullets|ParticleSystem|GetbUseLocalSpace) (Variables|Bullets|Parameters|GetBulletLifetime) (Variables|Bullets|Parameters|GetBulletSize) (Variables|Bullets|Parameters|GetBulletCollisionSize)))
  (Variables|Default|SetBulletEmitter _returnvalue)
  (if (> _bulletspawnrate 0.0)
    (bind _returnvalue_2 (Utilities|Time|SetTimerbyFunctionName self "SpawnTimerExpired" (/ 1.0 _bulletspawnrate) true))
    (Variables|State|SetBulletSpawnTimerHandle _returnvalue_2)))

(event Custom|SpawnTimerExpired
  (if (Components|Activation|IsActive)
    (Class|S3DParticleSystemComponent|SpawnBulletfromActor (Variables|Default|GetBulletEmitter) (Components|GetOwner) (Variables|Bullets|Parameters|GetBulletVelocity))))