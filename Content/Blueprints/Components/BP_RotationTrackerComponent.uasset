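; Component that tracks how far a rotation has turned and fires a RotationThresholdExceeded event for each threshold-sized step.
; TrackRotation, while active, accumulates the angle between successive forward vectors using a dot product and arccosine.
; On crossing the threshold, it loops through the steps, passing each event a shortest-path lerp from the last stored rotation.
; The remainder carries over, and the owner's rotation is stored for the next crossing.
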(event Custom|Event%20TrackRotation
  (params (NewParam :type Rotator))
  (bind _returnvalue (Math|Vector|GetForwardVector NewParam))
  (bind _rotationthreshold (Variables|Stats|GetRotationThreshold))
  (if (Components|Activation|IsActive)
    (bind _output_get (Variables|State|SetRotationAccumulator (+ (Variables|State|GetRotationAccumulator) (Class|KismetMathLibrary|DegAcos (Math|Vector|DotProduct _returnvalue (Variables|State|GetLastForwardVector))))))
    (Variables|State|SetLastForwardVector _returnvalue)
    (if (> (+ _output_get (Variables|State|GetLeftoverRotation)) (Variables|Stats|GetRotationThreshold))
      (if (> (Variables|State|GetLeftoverRotation) 0.0)
        (Variables|State|SetFirstIndex 1)
        (Variables|State|SetRotationAccumulator (+ (Variables|State|GetLeftoverRotation) (Variables|State|GetRotationAccumulator)))
        (Variables|State|SetLeftoverRotation 0.0)
        (else
          (Variables|State|SetFirstIndex 0)))
      (for _index (range (Variables|State|GetFirstIndex) (Math|Float|Truncate (/ (- (Variables|State|GetRotationAccumulator) (Math|Float|%(Float) (Variables|State|GetRotationAccumulator) _rotationthreshold)) _rotationthreshold)))
        (Default|CallRotationThresholdExceeded (Math|Rotator|Lerp(Rotator) (Variables|State|GetLastRotation) "0, 0, 0" (/ (* _index (Variables|Stats|GetRotationThreshold)) (Variables|State|GetRotationAccumulator)) true)))
      (Variables|State|SetLeftoverRotation (Math|Float|%(Float) (Variables|State|GetRotationAccumulator) _rotationthreshold))
      (Variables|State|SetRotationAccumulator 0.0)
      (Variables|State|SetLastRotation (Transformation|GetActorRotation (Components|GetOwner))))))