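; Enemy movement component that drives its owner's control input with a sine wave based on time since activation.
; On the X axis it pulses input along the cached forward vector using the absolute sine, so motion never reverses.
; On Y or Z it swings the actor's forward vector around the cached right or up vector by a sine-scaled angle.
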(fn CalculateControlInput
  (params (DeltaTime :type Float%20%28single-precision%29))
  (bind _returnvalue (Class|S3DEnemyMovementComponent|GetSecondsSinceActivation))
  (bind _cachedorientation (Variables|Default|GetCachedOrientation))
  (bind _sinefrequency (Variables|SineMovement|GetSineFrequency))
  (bind _returnvalue_2 (* _returnvalue _sinefrequency))
  (bind _returnvalue_3 (Math|Trig|Sin(Degrees) _returnvalue_2))
  (switch Utilities|FlowControl|Switch|SwitchonESplineMeshAxis (Variables|SineMovement|GetSineAxis)
    (:X
      (return (* (Math|Vector|GetForwardVector _cachedorientation) (Math|Float|Absolute(Float) _returnvalue_3))))
    (:Y
      (LocalVariables|SetRotationAxis (Math|Vector|GetRightVector _cachedorientation)))
    (:Z
      (LocalVariables|SetRotationAxis (Math|Vector|GetUpVector _cachedorientation))))
  (return (Math|Vector|RotateVectorAroundAxis (Transformation|GetActorForwardVector (Components|GetOwner)) (* _returnvalue_3 (Variables|SineMovement|GetSineAngle)) (LocalVariables|GetRotationAxis))))