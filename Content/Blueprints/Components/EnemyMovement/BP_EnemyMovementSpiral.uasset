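; BP_EnemyMovementSpiral is an enemy movement component that steers its enemy along a spiralling path around a cached forward direction.
; CalculateControlInput swings that forward vector about the cached right axis by a sine of time since activation and about the up axis by a cosine.
; It returns the normalized sum of both rotated vectors as control input, with frequency and angle variables shaping the spiral.
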(event EventBeginPlay)

(event EventTick
  (params (DeltaSeconds :type Float%20%28single-precision%29)))

(fn CalculateControlInput
  (params (DeltaTime :type Float%20%28single-precision%29))
  (bind _returnvalue (Class|S3DEnemyMovementComponent|GetSecondsSinceActivation))
  (bind _cachedorientation (Variables|Default|GetCachedOrientation))
  (bind _sinefrequency (Variables|SineMovement|GetSineFrequency))
  (bind _sineangle (Variables|SineMovement|GetSineAngle))
  (bind _returnvalue_2 (Math|Vector|GetForwardVector _cachedorientation))
  (bind _returnvalue_3 (* _returnvalue _sinefrequency))
  (return (Math|Vector|Normalize (+ (Math|Vector|RotateVectorAroundAxis _returnvalue_2 (* (Math|Trig|Sin(Degrees) _returnvalue_3) _sineangle) (Math|Vector|GetRightVector _cachedorientation)) (Math|Vector|RotateVectorAroundAxis _returnvalue_2 (* (Math|Trig|Cos(Degrees) _returnvalue_3) _sineangle) (Math|Vector|GetUpVector _cachedorientation))))))