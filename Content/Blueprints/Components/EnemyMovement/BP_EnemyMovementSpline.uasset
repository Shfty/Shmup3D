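; Enemy movement component that carries its owner along a spawned spline path toward the play volume.
; On activation it spawns a BP_SplineActor at the owner with a two-point, fixed-duration spline, replacing any existing path on reset.
; Each tick it re-pins the end point to the play volume's current location and sets the owner's transform by elapsed time.
; CalculateControlInput returns zero, since movement is set directly.
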(event Custom|ComponentActivated
  (params (bReset :type Boolean))
  (bind _returnvalue (Components|GetOwner))
  (if bReset
    (Variables|Default|SetTimeAlongSpline 0.0)
    (Utilities|IsValid (Variables|Default|GetSplinePath)
      (:Is%20Valid
        (Actor|DestroyActor (Variables|Default|GetSplinePath)))
      (:Is%20Not%20Valid
        _))
    (else
      (Utilities|IsValid (Variables|Default|GetSplinePath)
        (:Is%20Not%20Valid
          _))))
  (bind _returnvalue_2 (Game|SpawnActorfromClass "/Game/Blueprints/Environment/BP_SplineActor.BP_SplineActor_C" (Transformation|GetActorTransform _returnvalue) "AlwaysSpawn" _returnvalue 0))
  (bind _output_get (Variables|Default|SetSplinePath _returnvalue_2))
  (Spline|ClearSplinePoints (Variables|/Game/Blueprints/Environment/BP_SplineActor.BP_SplineActor_C|GetSpline _output_get) false)
  (Spline|AddSplinePoint (Variables|/Game/Blueprints/Environment/BP_SplineActor.BP_SplineActor_C|GetSpline _output_get) (Math|Vector|MakeVector 0.0 0.0 0.0) "Local" false)
  (Spline|AddSplinePoint (Variables|/Game/Blueprints/Environment/BP_SplineActor.BP_SplineActor_C|GetSpline _output_get) (Transformation|GetActorLocation (CallFunction|GetPlayVolume)) "World" true)
  (Variables|/Script/Engine.SplineComponent|SetDuration (Variables|/Game/Blueprints/Environment/BP_SplineActor.BP_SplineActor_C|GetSpline _output_get) 5.0))

(event EventTick
  (params (DeltaSeconds :type Float%20%28single-precision%29))
  (bind _splinepath (Variables|Default|GetSplinePath))
  (bind _timealongspline (Variables|Default|GetTimeAlongSpline))
  (bind _spline (Variables|/Game/Blueprints/Environment/BP_SplineActor.BP_SplineActor_C|GetSpline _splinepath))
  (bind _returnvalue (Spline|GetTransformatTime _spline _timealongspline "World" false false))
  (|CallParentFunction DeltaSeconds)
  (Utilities|IsValid _splinepath
    (:Is%20Valid
      (Spline|SetLocationatSplinePoint _spline 1 (Transformation|GetActorLocation (CallFunction|GetPlayVolume)) "World" true)
      (Transformation|SetActorTransform (Components|GetOwner) (Math|Transform|MakeTransform (.location _returnvalue) (.rotation _returnvalue) "1,1,1"))
      (CallFunction|AddFloatbyReference (Variables|Default|GetTimeAlongSpline) DeltaSeconds))))

(event EventBeginPlay
  (EventDispatchers|BindEventtoOnComponentActivated (EventDispatchers|CreateEvent :!event Custom|ComponentActivated))
  (|CallParentFunction))

(fn CalculateControlInput
  (params (DeltaTime :type Float%20%28single-precision%29))
  (return "0, 0, 0"))