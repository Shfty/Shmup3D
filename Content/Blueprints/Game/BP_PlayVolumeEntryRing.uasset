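; BP_PlayVolumeEntryRing is a short-lived ring effect actor, named for play volume entry, that grows and then expires.
; On BeginPlay it creates a dynamic material on PlaneMesh, passes it the Duration and sets its lifespan to match.
; Each Tick scales the plane up by ScaleRate and feeds normalized age to the material's Time parameter, letting the material animate over the actor's life.
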(event EventTick
  (params (DeltaSeconds :type Float%20%28single-precision%29))
  (bind _planemesh (Variables|Default|GetPlaneMesh))
  (Transformation|SetRelativeScale3D _planemesh (+ (Variables|/Script/Engine.SceneComponent|GetRelativeScale3D _planemesh) (* DeltaSeconds (Variables|Default|GetScaleRate))))
  (Rendering|Material|SetScalarParameterValue (Variables|Default|GetMaterialInstance) "Time" (/ (Actor|GetGameTimeSinceCreation) (Variables|Actor|GetInitialLifeSpan)) :!class /Script/Engine.MaterialInstanceDynamic))

(event EventBeginPlay
  (bind _duration (Variables|Default|GetDuration))
  (bind _planemesh (Variables|Default|GetPlaneMesh))
  (bind _returnvalue (Rendering|Material|CreateDynamicMaterialInstance _planemesh 0 (Rendering|Material|GetMaterial _planemesh 0) :!class /Script/Engine.PrimitiveComponent))
  (bind _output_get (Variables|Default|SetMaterialInstance _returnvalue))
  (Rendering|Material|SetScalarParameterValue _output_get "Duration" _duration :!class /Script/Engine.MaterialInstanceDynamic)
  (Actor|SetLifeSpan _duration))

(fn ConstructionScript)