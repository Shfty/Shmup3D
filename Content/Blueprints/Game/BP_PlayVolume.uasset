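; Moving play-area box that registers with the GameState, plays level sequences for intro, match and outro, and hosts a radar scene capture.
; On match start it shows its bounds, starts the sequence, registers tagged player and volume components with the radar, and enables tick.
; Tick yaws the radar spring arm with control rotation, syncs sequence rate to time dilation, and follows a spline, using spline point X scale as speed.
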(event Custom|DevelopmentOnly
  (Variables|Stats|SetIntroSequence 0))

(event EventTick
  (params (DeltaSeconds :type Float%20%28single-precision%29))
  (bind _sequenceplayer (Variables|State|GetSequencePlayer))
  (bind _splinepath (Variables|Default|GetSplinePath))
  (bind _spline (Variables|/Game/Blueprints/Environment/BP_SplineActor.BP_SplineActor_C|GetSpline _splinepath))
  (Utilities|FlowControl|Sequence
    (:then_0
      ;[1 1 1] Set scene capture spring arm orientation
      (Transformation|SetWorldRotation (Variables|Default|GetSpringArm) (Math|Rotator|CombineRotators (Math|Rotator|MakeRotator 0.0 -35.265 0.0) (Math|Rotator|MakeRotator 0.0 0.0 (.yaw (Pawn|GetControlRotation (Game|GetPlayerController 0) :!class /Script/Engine.Controller)))) false false))
    (:then_1
      ;[1 1 1] Make sequence player respect time dilation
      (Utilities|IsValid _sequenceplayer
        (:Is%20Valid
          (Components|Timeline|SetPlayRate _sequenceplayer (Class|GameplayStatics|GetGlobalTimeDilation)))))
    (:then_2
      ;[1 1 1] Travel along spline path
      (Utilities|IsValid _splinepath
        (:Is%20Valid
          (Transformation|SetActorTransform (Math|Transform|MakeTransform (.location (Spline|GetTransformatDistanceAlongSpline _spline (Variables|Default|GetDistanceAlongSpline) "World" false)) (.rotation (Spline|GetTransformatDistanceAlongSpline _spline (Variables|Default|GetDistanceAlongSpline) "World" false)) "1,1.000000,1") false true)
          (Variables|Default|SetDistanceAlongSpline (+ (Variables|Default|GetDistanceAlongSpline) (* (Utilities|Time|GetWorldDeltaSeconds) (.x (Class|SplineComponent|GetScaleatDistanceAlongSpline _spline (Variables|Default|GetDistanceAlongSpline)))))))))))

(event EventBeginPlay
  (Default|CheckinPlayVolume (CallFunction|GetGameState) self)
  (Rendering|SetVisibility (Variables|Default|GetBounds) false true)
  (CallFunction|DevelopmentOnly))

(event EventMatchStarted
  (bind _playerpawn (CallFunction|GetPlayerPawn))
  (bind _radarcomponenttag (Variables|Stats|GetRadarComponentTag))
  (Utilities|FlowControl|Sequence
    (:then_0
      (Rendering|SetVisibility (Variables|Default|GetBounds) true true))
    (:then_1
      (bind _returnvalue (Sequencer|Player|CreateLevelSequencePlayer (Variables|Stats|GetLevelSequence) (Utilities|Struct|MakeLevelSequencePlaybackSettings 0 0.8)))
      (Utilities|IsValid _returnvalue
        (:Is%20Valid
          (Variables|State|SetSequencePlayer _returnvalue)
          (Audio|Components|Audio|Play _returnvalue))))
    (:then_2
      (Utilities|IsValid _playerpawn
        (:Is%20Valid
          (Utilities|AddRadarShownComponents (Actor|GetComponentsbyTag _playerpawn "/Script/Engine.PrimitiveComponent" _radarcomponenttag)
            (:Out
              (Utilities|AddRadarShownComponents (Actor|GetComponentsbyTag "/Script/Engine.PrimitiveComponent" _radarcomponenttag)))))))
    (:then_3
      (Actor|Tick|SetActorTickEnabled true))))

(fn ConstructionScript
  (bind _returnvalue (Rendering|Material|CreateDynamicMaterialInstance "/Game/Materials/M_PlayVolume.M_PlayVolume" :!class /Script/Engine.KismetMaterialLibrary))
  (Rendering|Material|SetVectorParameterValue _returnvalue "EmissiveColor" (Variables|Stats|GetColor) :!class /Script/Engine.MaterialInstanceDynamic)
  (Rendering|Material|SetMaterial (Variables|Default|GetCeiling) 0 _returnvalue)
  (Components|Box|SetBoxExtent (Variables|Default|GetBounds) (* (Math|Conversions|ToVector(Float) (Variables|Stats|GetVolumeSize)) 0.5) false)
  (Transformation|SetRelativeScale3D (Variables|Default|GetFaces) (Math|Conversions|ToVector(Float) (Variables|Stats|GetVolumeSize))))

(fn PlayIntroSequence
  (bind _introsequence (Variables|Stats|GetIntroSequence))
  (Utilities|IsValid _introsequence
    (:Is%20Valid
      (bind _returnvalue (Sequencer|Player|CreateLevelSequencePlayer _introsequence (Utilities|Struct|MakeLevelSequencePlaybackSettings 0 1.0)))
      (Utilities|IsValid _returnvalue
        (:Is%20Valid
          (Variables|State|SetSequencePlayer _returnvalue)
          (Audio|Components|Audio|Play _returnvalue)
          (return true))
        (:Is%20Not%20Valid
          (return false))))
    (:Is%20Not%20Valid
      (return false))))

(fn PlayOutroSequence
  (bind _returnvalue (Sequencer|Player|CreateLevelSequencePlayer (Variables|Stats|GetOutroSequence) (Utilities|Struct|MakeLevelSequencePlaybackSettings 0 1.0)))
  (Utilities|IsValid _returnvalue
    (:Is%20Valid
      (Variables|State|SetSequencePlayer _returnvalue)
      (Audio|Components|Audio|Play _returnvalue)
      (return))
    (:Is%20Not%20Valid
      (return))))