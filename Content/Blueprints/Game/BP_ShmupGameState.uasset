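; Game state for a shmup that tracks the play volume, the enemies inside it and the active boss.
; Enemy entry and exit update the list and radar scene capture, play a sound and spawn a ring on the volume's bounds.
; Hitstop drops global time dilation to near zero, with Tick counting down in real time to restore it.
; A development-only event on BeginPlay mutes the music sound class.
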(event Custom|Event%20DevelopmentOnly
  (Audio|SetSoundMixClassOverride "/Game/Sounds/DefaultSoundMix.DefaultSoundMix" "/Game/Sounds/SoundClasses/SC_Music.SC_Music" 0.0 1.0 0.0 true))

(event Custom|Event%20BossActivated
  (params (Boss :type BP%20Boss%20Object%20Reference))
  (Variables|Bosses|SetActiveBoss Boss))

(event Custom|Event%20BossDefeated
  (params (Boss :type BP%20Boss%20Object%20Reference))
  (Variables|Bosses|SetActiveBoss 0))

(event Custom|Event%20Hitstop
  (params (Frames :type Integer))
  ;[1 1 1] Hitstop handlers
  (if (and (> Frames 0) (== (Variables|Default|GetHitstopAccumulator) 0.0))
    (Variables|Default|SetHitstopAccumulator (/ (Math|Conversions|ToFloat(Integer) Frames) (Math|Float|MakeLiteralFloat 6e+01)))
    (Utilities|Time|SetGlobalTimeDilation (Math|Float|MakeLiteralFloat 0.0001))))

(event Custom|CheckInPlayVolume
  (params (PlayVolume :type Actor%20Object%20Reference))
  (Variables|Default|SetPlayVolume PlayVolume))

(event EventBeginPlay
  (CallFunction|EventDevelopmentOnly))

(event EventTick
  (params (DeltaSeconds :type Float%20%28single-precision%29))
  (bind _returnvalue (Utilities|Time|GetRealTimeSeconds))
  ;[1 1 1] Hitstop handlers
  (Utilities|FlowControl|Sequence
    (:then_0
      (if (> (Variables|Default|GetHitstopAccumulator) 0.0)
        (bind _output_get (Variables|Default|SetHitstopAccumulator (- (Variables|Default|GetHitstopAccumulator) (- _returnvalue (Variables|Default|GetLastRealTimeSeconds)))))
        (if (<= _output_get 0.0)
          (Utilities|Time|SetGlobalTimeDilation 1.0)
          (Variables|Default|SetHitstopAccumulator 0.0))))
    (:then_1
      (Variables|Default|SetLastRealTimeSeconds _returnvalue))))

(fn ConstructionScript)

(fn EnemyEnteredPlayVolume
  (params (Enemy :type BP%20Enemy%20Object%20Reference))
  (bind _playvolume (CallFunction|GetPlayVolume))
  (bind _returnvalue (Transformation|GetActorLocation Enemy))
  (bind _returnvalue_2 (Actor|GetComponentsByClass Enemy "/Game/Blueprints/Components/BP_BulletSpawnerComponent.BP_BulletSpawnerComponent_C"))
  (bind _radarscenecapture (Variables|/Game/Blueprints/Game/BP_PlayVolume.BP_PlayVolume_C|GetRadarSceneCapture _playvolume))
  (Utilities|Array|AddUnique (Variables|Default|GetEnemiesInPlayVolume) Enemy)
  (Rendering|SceneCapture|ShowOnlyActorComponents _radarscenecapture Enemy)
  (if (> (Utilities|Array|Length _returnvalue_2) 0)
    (Rendering|SceneCapture|ShowOnlyComponent _radarscenecapture (Variables|/Game/Blueprints/Components/BP_BulletSpawnerComponent.BP_BulletSpawnerComponent_C|GetBulletEmitter (Utilities|Array|Get(acopy) _returnvalue_2))))
  (PlayVolume|SpawnPlayVolumeRing _returnvalue)
  (Audio|PlaySoundatLocation (Variables|PlayVolume|GetPlayVolumeEntrySound) _returnvalue))

(fn EnemyLeftPlayVolume
  (params (Enemy :type BP%20Enemy%20Object%20Reference))
  (bind _returnvalue (Transformation|GetActorLocation Enemy))
  (PlayVolume|RemoveEnemyfromPlay Enemy)
  (Class|SceneCaptureComponent|HideActorComponents (Variables|/Game/Blueprints/Game/BP_PlayVolume.BP_PlayVolume_C|GetRadarSceneCapture (CallFunction|GetPlayVolume)) Enemy)
  (PlayVolume|SpawnPlayVolumeRing _returnvalue)
  (Audio|PlaySoundatLocation (Variables|PlayVolume|GetPlayVolumeExitSound) _returnvalue))

(fn SpawnPlayVolumeRing
  (params (Location :type Vector))
  (bind _returnvalue (Game|SpawnActorfromClass "/Game/Blueprints/Game/BP_PlayVolumeEntryRing.BP_PlayVolumeEntryRing_C" (Math|Transform|MakeTransform (.OutPointOnBody (Collision|GetClosestPointonCollision (Variables|/Game/Blueprints/Game/BP_PlayVolume.BP_PlayVolume_C|GetBounds (.AsBP%20Play%20Volume (Utilities|Casting|CastToBP_PlayVolume (Variables|Default|GetPlayVolume)))) Location "None")) "0, 0, 0" "1.000000,1,1") "AlwaysSpawn" 0 1.0 1e+03))
  (Utilities|IsValid _returnvalue
    (:Is%20Valid
      (Transformation|AttachActorToActor _returnvalue (.AsBP%20Play%20Volume (Utilities|Casting|CastToBP_PlayVolume (Variables|Default|GetPlayVolume))) "None" "KeepWorld" "KeepRelative" "KeepWorld" false)
      (return))
    (:Is%20Not%20Valid
      (return))))

(fn RemoveEnemyfromPlay
  (params (Enemy :type BP%20Enemy%20Object%20Reference))
  (bind _enemiesinplayvolume (Variables|Default|GetEnemiesInPlayVolume))
  (if (Utilities|Array|ContainsItem _enemiesinplayvolume Enemy)
    (Utilities|Array|RemoveItem _enemiesinplayvolume Enemy)
    (return)
    (else
      (return))))