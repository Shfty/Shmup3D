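; BP_LookAtCamera is an actor, named as a camera, that keeps itself rotated to face a TargetActor.
; A shared LookAtTarget function computes the look-at rotation from its own location to the target's and applies it, skipping when the target is invalid.
; It runs from the Construction Script, so the aim also updates on construction, and on every Tick, so it follows the target at runtime.
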(event EventTick
  (params (DeltaSeconds :type Float%20%28single-precision%29))
  (CallFunction|LookatTarget))

(fn ConstructionScript
  (CallFunction|LookatTarget))

(fn LookatTarget
  (bind _targetactor (Variables|Default|GetTargetActor))
  (Utilities|IsValid _targetactor
    (:Is%20Valid
      (Transformation|SetActorRotation (Math|Rotator|FindLookatRotation (Transformation|GetActorLocation) (Transformation|GetActorLocation _targetactor))))
    (:Is%20Not%20Valid
      _))
  (return))