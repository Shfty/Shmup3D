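; Shoot 'em up game mode that starts the match immediately and runs the opening hand-off to the player.
; When the match goes In Progress, it asks the play volume to play its intro sequence, calling IntroFinished directly if none plays.
; IntroFinished blends the camera to the player pawn, possesses it after the blend, then notifies every actor implementing the match-started interface.
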(event Custom|Event%20IntroFinished
  (bind _returnvalue (Game|GetPlayerController 0))
  (bind _gamestartcamerablendtime (Variables|Default|GetGameStartCameraBlendTime))
  (bind _asbp_shmup_player_controller (Utilities|Casting|CastToBP_ShmupPlayerController _returnvalue))
  ;[1 1 1] Match start handler
  (bind _outactors (Actor|GetAllActorsOfClass "/Game/Blueprints/Player/BP_ShmupPlayerPawn.BP_ShmupPlayerPawn_C"))
  (Game|Player|SetViewTargetwithBlend _asbp_shmup_player_controller (Utilities|Array|Get(acopy) _outactors) _gamestartcamerablendtime "VTBlend_Cubic" 1.0 true)
  (Utilities|FlowControl|Delay _gamestartcamerablendtime)
  (Pawn|Possess _asbp_shmup_player_controller (Utilities|Array|Get(acopy) _outactors))
  (bind _outactors_2 (Actor|GetAllActorswithInterface "/Game/Blueprints/Interfaces/BP_MatchStartedInterface.BP_MatchStartedInterface_C"))
  (for _array_element _outactors_2
    (Class|BPMatchStartedInterface|MatchStarted(Message) _array_element)))

(event EventOnSetMatchState
  (params (NewState :type Name))
  (bind _gamestate (CallFunction|GetGameState))
  (bind _playvolume (Variables|/Script/Shmup3D.S3DGameState|GetPlayVolume _gamestate))
  (bind _asbp_play_volume (Utilities|Casting|CastToBP_PlayVolume _playvolume))
  (switch name NewState
    (:InProgress
      ;[1 1 1] Match start handler
      (Utilities|IsValid _asbp_play_volume
        (:Is%20Valid
          (bind _success (Default|PlayIntroSequence _asbp_play_volume))
          (if (not _success)
            (CallFunction|EventIntroFinished :!label _label)))
        (:Is%20Not%20Valid
          (goto _label))))))

(fn ConstructionScript)

(fn ReadytoStartMatch
  (return true))