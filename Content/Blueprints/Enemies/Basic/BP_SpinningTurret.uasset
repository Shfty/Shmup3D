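; BP_SpinningTurret is an enemy turret that continuously spins its mesh and fires bullet bursts as it turns.
; Tick rotates the mesh around a configurable axis and feeds its world rotation to RotationTracker.
; When the tracker's threshold is exceeded and BulletSpawner is active, its emitter fires a central bullet from the mesh transform.
; Additional subdivision bullets fire at angular offsets derived from the cone angle, around a configurable axis.
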(event RotationThresholdExceeded(RotationTracker)
  (params (Rotation :type Rotator))
  (bind _returnvalue (* "0.000000, 0,1.000000" 2.5e+03))
  (bind _mesh (Variables|Default|GetMesh))
  (bind _bulletstreamconeangle (Variables|Default|GetBulletStreamConeAngle))
  (bind _returnvalue_2 (Transformation|GetWorldTransform _mesh))
  (Utilities|IsValid self
    (:Is%20Valid
      (if (Components|Activation|IsActive (Variables|Default|GetBulletSpawner))
        (Class|S3DParticleSystemComponent|SpawnBulletatTransform (Variables|/Game/Blueprints/Components/BP_BulletSpawnerComponent.BP_BulletSpawnerComponent_C|GetBulletEmitter (Variables|Default|GetBulletSpawner)) _returnvalue_2 _returnvalue)
        (for _index (range 0 (- (Variables|Default|GetBulletStreamSubdivisions) 2))
          (Class|S3DParticleSystemComponent|SpawnBulletatTransform (Variables|/Game/Blueprints/Components/BP_BulletSpawnerComponent.BP_BulletSpawnerComponent_C|GetBulletEmitter (Variables|Default|GetBulletSpawner)) _returnvalue_2 (Math|Vector|RotateVectorAroundAxis _returnvalue (+ (* _index (* _bulletstreamconeangle 2.0)) (* _bulletstreamconeangle -1.0)) (Variables|Default|GetBulletStreamSubdivisionAxis))))))))

(event EventTick
  (params (DeltaSeconds :type Float%20%28single-precision%29))
  (Utilities|IsValid self
    (:Is%20Valid
      (CallFunction|Spin DeltaSeconds)
      (Default|EventTrackRotation (Variables|Default|GetRotationTracker) (Transformation|GetWorldRotation (Variables|Default|GetMesh)))
      (|CallParentFunction DeltaSeconds))))

(fn ConstructionScript
  (|CallParentFunction))

(fn Spin
  (params (DeltaSeconds :type Float%20%28single-precision%29))
  (Transformation|AddWorldRotation (Variables|Default|GetMesh) (Math|Vector|RotatorfromAxisandAngle (Math|Vector|Normalize (Variables|Rotation|GetRotationAxis)) (* (Variables|Rotation|GetRotationRate) DeltaSeconds)) false false)
  (return))