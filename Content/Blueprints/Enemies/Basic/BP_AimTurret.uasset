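; BP_AimTurret is a basic shmup enemy turret that turns its whole actor to face the player's pawn.
; Each Tick it snaps its X axis toward the cached player location without interpolation, then calls the parent Tick.
; When the reference is invalid, it caches player 0's pawn as BP_ShmupPlayerPawn and skips rotation that frame.
; A failed cast also skips the parent Tick.
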(event EventTick
  (params (DeltaSeconds :type Float%20%28single-precision%29))
  (Utilities|IsValid (Variables|Default|GetPlayerPawn)
    (:Is%20Valid
      (Transformation|SetActorRotation (Math|Rotator|MakeRotfromX (- (Transformation|GetActorLocation (Variables|Default|GetPlayerPawn)) (Transformation|GetActorLocation)))))
    (:Is%20Not%20Valid
      (bind _asbp_shmup_player_pawn (Utilities|Casting|CastToBP_ShmupPlayerPawn (Game|Player|GetPlayerPawn 0)))
      (Variables|Default|SetPlayerPawn _asbp_shmup_player_pawn)))
  (|CallParentFunction DeltaSeconds))

(fn ConstructionScript
  (|CallParentFunction))