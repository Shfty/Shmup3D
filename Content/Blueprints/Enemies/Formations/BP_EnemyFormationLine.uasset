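; Enemy formation Blueprint that lays out formation slots in a straight line.
; The construction script rebuilds ActorTransforms with LineSubdivisions evenly spaced entries, then runs the parent construction script.
; Each index maps to an offset from -1 to 1, which MakeLineFormationTransform scales by LineSize along X, so LineSize is the half-length of the centered line.
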(fn ConstructionScript
  (bind _actortransforms (Variables|Default|GetActorTransforms))
  (bind _linesubdivisions (Variables|LineFormation|GetLineSubdivisions))
  (bind _returnvalue (- _linesubdivisions 1))
  (Utilities|Array|Clear _actortransforms)
  (for _index (range 0 _returnvalue)
    (Utilities|Array|Add _actortransforms (CallFunction|MakeLineFormationTransform (* (- (/ (Math|Conversions|ToFloat(Integer) _index) (Math|Conversions|ToFloat(Integer) _returnvalue)) 0.5) 2.0))))
  (|CallParentFunction))

(fn MakeLineFormationTransform
  (params (Offset :type Float%20%28single-precision%29))
  (return (CallFunction|MakeFormationTransform (Math|Vector|MakeVector (* Offset (Variables|LineFormation|GetLineSize)) 0.0 0.0))))