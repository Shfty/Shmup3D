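; BP_EnemyFormationCross is an enemy formation that defines four slots at the diagonal corners of a square in the local YZ plane.
; The construction script fills ActorTransforms before running the parent's construction script.
; MakeCrossFormationTransform scales each unit corner offset by CrossSize and passes it to MakeFormationTransform with zero X.
; The event graph holds no active logic.
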(event EventBeginPlay
  (|CallParentFunction))

(event Collision|EventActorBeginOverlap
  (params (OtherActor :type Actor%20Object%20Reference)))

(event EventTick
  (params (DeltaSeconds :type Float%20%28single-precision%29)))

(fn ConstructionScript
  (Variables|Default|SetActorTransforms (Utilities|Array|MakeArray (CallFunction|MakeCrossFormationTransform (Math|Vector2D|MakeVector2D -1.0 1.0)) (CallFunction|MakeCrossFormationTransform (Math|Vector2D|MakeVector2D 1.0 1.0)) (CallFunction|MakeCrossFormationTransform (Math|Vector2D|MakeVector2D -1.0 -1.0)) (CallFunction|MakeCrossFormationTransform (Math|Vector2D|MakeVector2D 1.0 -1.0))))
  (|CallParentFunction))

(fn MakeCrossFormationTransform
  (params (A :type Vector%202D%20Structure))
  (bind _crosssize (Variables|CrossFormation|GetCrossSize))
  (bind _returnvalue (* A _crosssize))
  (return (CallFunction|MakeFormationTransform (Math|Vector|MakeVector 0.0 (.x _returnvalue) (.y _returnvalue)))))