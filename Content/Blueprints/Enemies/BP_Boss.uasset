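; Boss enemy assembled from child-actor enemies that acts as one opponent with combined health.
; At match start it initializes each child enemy and binds to its damage event, re-summing their health on every hit and dying at zero.
; Entering the play volume reports boss activation to the GameState; removal or leaving the volume reports defeat.
; Its own damage events are empty, as are the activation, defeat and death-effect events.
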(event Custom|Event%20ComponentEnemyTookDamage
  (params (DamagedActor :type Actor%20Object%20Reference) (Damage :type Float%20%28single-precision%29) (DamageType :type Damage%20Type%20Object%20Reference) (InstigatedBy :type Controller%20Object%20Reference) (DamageCauser :type Actor%20Object%20Reference))
  (if (> (Variables|Default|GetHealth) 0)
    (Variables|Default|SetHealth 0)
    (for _array_element (Variables|Default|GetComponentEnemies)
      (Variables|Default|SetHealth (+ (Variables|Default|GetHealth) (Variables|/Game/Blueprints/Enemies/BP_Enemy.BP_Enemy_C|GetHealth _array_element))))
    (if (<= (Variables|Default|GetHealth) 0)
      (CallFunction|EnemyDeath))))

(event Custom|BossActivated)

(event Custom|BossDefeated)

(event EventRemoveSelffromPlay
  (bind _gamestate (CallFunction|GetGameState))
  (bind _self self)
  (Default|EventBossDefeated _gamestate _self)
  (Default|CallBossDefeated _gamestate _self)
  (CallFunction|BossDefeated))

(event EventEnterPlayVolume
  (bind _gamestate (CallFunction|GetGameState))
  (bind _self self)
  (Default|EventBossActivated _gamestate _self)
  (Default|CallBossActivated _gamestate _self)
  (CallFunction|BossActivated))

(event EventLeavePlayVolume
  (bind _gamestate (CallFunction|GetGameState))
  (bind _self self)
  (Default|EventBossDefeated _gamestate _self)
  (Default|CallBossDefeated _gamestate _self)
  (CallFunction|BossDefeated))

(event EventMatchStarted
  (|CallParentFunction)
  (for _array_element (Actor|GetComponentsByClass self "/Script/Engine.ChildActorComponent")
    (bind _asbp_enemy (Utilities|Casting|CastToBP_Enemy (Variables|/Script/Engine.ChildActorComponent|GetChildActor _array_element)))
    (Utilities|Array|AddUnique (Variables|Default|GetComponentEnemies) _asbp_enemy)
    (Default|InitializeEnemy _asbp_enemy)
    (EventDispatchers|AssignOnTakeAnyDamage _asbp_enemy (delegate Custom|Event%20ComponentEnemyTookDamage))))

(event Game|Damage|EventAnyDamage
  (params (Damage :type Float%20%28single-precision%29) (DamageType :type Damage%20Type%20Object%20Reference) (InstigatedBy :type Controller%20Object%20Reference) (DamageCauser :type Actor%20Object%20Reference)))

(event EventEnemyDeath
  (CallFunction|PlayDeathEffects)
  (CallFunction|RemoveSelffromPlay))

(event EventPlayDeathEffects)

(event EventTakeDamage
  (params (Damage :type Float%20%28single-precision%29) (DamageType :type Damage%20Type%20Object%20Reference)))

(fn ConstructionScript
  (|CallParentFunction))