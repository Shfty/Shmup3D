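; Enemy formation actor that spawns a set of child enemies of a chosen class and passes its ActivationDistance to each on BeginPlay.
; Construction feeds class and editor folder to the parent script, recovering a lost EnemyClass from the first child as a partial workaround.
; It places an indicator sphere at that distance along the play volume path spline.
; MakeFormationTransform orients members along a facing vector or toward it as a look-at point.
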(event EventBeginPlay
  (for _array_element (Variables|Default|GetChildActorComponents)
    (bind _asbp_enemy (Utilities|Casting|CastToBP_Enemy (Variables|/Script/Engine.ChildActorComponent|GetChildActor _array_element)))
    (Variables|/Game/Blueprints/Enemies/BP_Enemy.BP_Enemy_C|SetActivationDistance _asbp_enemy (Variables|EnemyFormation|GetActivationDistance))))

(fn ConstructionScript
  (bind _childactorcomponents (Variables|Default|GetChildActorComponents))
  (bind _activationindicatorsphere (Variables|Default|GetActivationIndicatorSphere))
  (Utilities|FlowControl|Sequence
    (:then_0
      (if (!= (Variables|EnemyFormation|GetEnemyClass) 0)
        (bind _output_get (Variables|Default|SetActorClass (Variables|EnemyFormation|GetEnemyClass) :!label _label))
        (Variables|Default|SetFolderName (Utilities|String|StringToName (Utilities|String|Append "Enemy Formations/" (Utilities|GetClassDisplayName _output_get))))
        (|CallParentFunction)
        (else
          ;[1 1 1] Partial workaround for loss of instance data
          (if (> (Utilities|Array|Length _childactorcomponents) 0)
            (bind _asbp_enemy (Utilities|Casting|CastToBP_Enemy (Variables|/Script/Engine.ChildActorComponent|GetChildActor (Utilities|Array|Get(acopy) _childactorcomponents))))
            (Variables|EnemyFormation|SetEnemyClass (Utilities|GetClass _asbp_enemy))
            (goto _label)))))
    (:then_1
      (bind _outactors (Actor|GetAllActorsOfClass "/Game/Blueprints/Environment/BP_PlayVolumePath.BP_PlayVolumePath_C"))
      (if (and (> (Utilities|Array|Length _outactors) 0) (>= (Variables|EnemyFormation|GetActivationDistance) 0.0))
        (Transformation|SetWorldLocation _activationindicatorsphere (Spline|GetLocationatDistanceAlongSpline (Variables|/Game/Blueprints/Environment/BP_SplineActor.BP_SplineActor_C|GetSpline (Utilities|Array|Get(acopy) _outactors)) (Variables|EnemyFormation|GetActivationDistance) "World") false true)
        (else
          (Rendering|SetVisibility _activationindicatorsphere false true))))))

(fn MakeFormationTransform
  (params (Location :type Vector))
  (bind _facingvector (Variables|EnemyFormation|GetFacingVector))
  (if (Variables|EnemyFormation|GetFacingVectorAsLookAt)
    (LocalVariables|SetRotation (Math|Rotator|MakeRotfromX (- _facingvector Location)))
    (else
      (LocalVariables|SetRotation (Math|Rotator|MakeRotfromX _facingvector))))
  (return (Math|Transform|MakeTransform Location (LocalVariables|GetRotation))))