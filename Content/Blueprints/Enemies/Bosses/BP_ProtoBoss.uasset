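; Prototype boss built from component enemies, orbiting arms and a core, with total health summed from those parts at match start.
; A phase state machine idles, then after a delay randomly picks Spin Cycle or Core Beam, whose timelines drive arm orbit and bullets before returning to selection.
; Destroying the core halts both attacks and leaves arms firing while sine waves swing them.
; Beam firing is only a debug print.
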(event Custom|Event%20PhaseChanged
  (params (FromState :type Byte) (ToState :type Byte))
  ;[1 1 1] Phase Change Handler
  (Utilities|FlowControl|Sequence
    (:then_0
      (switch Utilities|FlowControl|Switch|SwitchonProtoBossPhases (Utilities|Enum|ByteToEnumProtoBossPhases FromState)) ; Phase Exit Handlers
    )
    (:then_1
      (switch Utilities|FlowControl|Switch|SwitchonProtoBossPhases (Utilities|Enum|ByteToEnumProtoBossPhases ToState) ; Phase Entry Handlers
        (:NewEnumerator0
          (|EnterPhase_Idle))
        (:NewEnumerator1
          (|EnterPhase_PhaseSelect))
        (:NewEnumerator2
          (|EnterPhase_SpinCycle))
        (:NewEnumerator3
          (|EnterPhase_CoreBeam))
        (:NewEnumerator4
          (|EnterPhase_CoreDestroyed))))))

(event Custom|Event%20CoreDestroyed
  ;[1 1 1] Core Destruction Handler
  (Audio|Components|Audio|Stop (Variables|Default|GetCoreBeam))
  (Utilities|Time|ClearandInvalidateTimerbyHandle (Variables|Default|GetPhaseChangeTimerHandle))
  (Utilities|EnterPhase "NewEnumerator4"))

(event Custom|SelectPhase
  ;[1 1 1] Phase Selection Handler
  (switch int (Math|Random|RandomIntegerinRange 0 1)
    (:0
      (Utilities|EnterPhase "NewEnumerator2"))
    (:1
      (Utilities|EnterPhase "NewEnumerator3"))))

(event EventEventActivateBullets
  ;[1 1 1] Bullet Activation Overrides
  (for _array_element (Variables|State|GetArms)
    (Default|EventActivateBullets _array_element)))

(event EventTick
  (params (DeltaSeconds :type Float%20%28single-precision%29))
  (Utilities|FlowControl|Sequence
    (:then_0
      ;[1 1 1] Phase Tick Handlers
      (switch Utilities|FlowControl|Switch|SwitchonProtoBossPhases (Utilities|Enum|ByteToEnumProtoBossPhases (Variables|/Script/ShiftyPlugin.SPStateMachineComponent|GetCurrentState (Variables|Default|GetPhaseStateMachine)))
        (:NewEnumerator4
          (CallFunction|TickPhaseCoreDestroyed))))
    (:then_1
      (CallFunction|UpdateArmOrbit DeltaSeconds))))

(event EventBossDefeated)

(event EventMatchStarted
  (|CallParentFunction)
  ;[1 1 1] Total up health from component enemies
  (Variables|Default|SetHealth 0)
  (for _array_element (Variables|Default|GetComponentEnemies)
    (bind _output_get (Variables|Default|SetHealth (+ (Variables|Default|GetHealth) (Variables|/Game/Blueprints/Enemies/BP_Enemy.BP_Enemy_C|GetHealth _array_element))))
    (Variables|Default|SetMaxHealth _output_get)
    ;[1 1 1] Assign typed component enemy variables
    (bind _asbp_proto_boss_arm (Utilities|Casting|CastToBP_ProtoBossArm _array_element)
      (:then
        (Utilities|Array|AddUnique (Variables|State|GetArms) _asbp_proto_boss_arm))
      (:CastFailed
        (bind _asbp_proto_boss_core (Utilities|Casting|CastToBP_ProtoBossCore _array_element))
        (Variables|State|SetCore _asbp_proto_boss_core))))
  (EventDispatchers|AssignCoreDestroyed (Variables|State|GetCore) (EventDispatchers|CreateEvent :!event Custom|Event%20CoreDestroyed)))

(event EventEventDeactivateBullets
  ;[1 1 1] Bullet Activation Overrides
  (for _array_element (Variables|State|GetArms)
    (Default|EventDeactivateBullets _array_element)))

(event EventBeginPlay
  (Utilities|FlowControl|Sequence
    (:then_0
      ;[1 1 1] Event Bindings
      (EventDispatchers|AssignOnStateChanged (Variables|Default|GetPhaseStateMachine) (EventDispatchers|CreateEvent :!event Custom|Event%20PhaseChanged)))
    (:then_2
      ;[1 1 1] Enter Intro State
      (Utilities|EnterPhase "NewEnumerator0"))))

(event EventBossActivated
  ;[1 1 1] Initialization
  (Utilities|EnterPhase "NewEnumerator1"))

(fn ConstructionScript
  (|CallParentFunction))

(fn SetArmOrientation
  (params (Angle :type Float%20%28single-precision%29))
  (bind _returnvalue (Transformation|GetActorForwardVector))
  (for _array_element (Variables|State|GetArms)
    (Transformation|SetWorldRotation (Variables|/Game/Blueprints/Enemies/BP_Enemy.BP_Enemy_C|GetRootScene _array_element) (Math|Rotator|CombineRotators (Math|Rotator|MakeRotfromX _returnvalue) (Math|Vector|RotatorfromAxisandAngle (Math|Vector|CrossProduct (Math|Vector|Normalize (- (Transformation|GetActorLocation _array_element) (Transformation|GetActorLocation))) _returnvalue) Angle)) false false)))

(fn UpdateArmOrbit
  (params (DeltaSeconds :type Float%20%28single-precision%29))
  (Transformation|AddRelativeRotation (Variables|Default|GetArmsScene) (Math|Rotator|MakeRotator (* DeltaSeconds (Variables|Stats|GetArmRotationSpeed)) 0.0 0.0) false false)
  (return))

(fn TickPhaseCoreDestroyed
  (bind _returnvalue (Utilities|Time|GetGameTimeinSeconds))
  (CallFunction|SetArmOrientation (* (Math|Trig|Sin(Degrees) (* _returnvalue 2e+02)) 3e+01))
  (Variables|Stats|SetArmRotationSpeed (* (Math|Trig|Sin(Degrees) (* _returnvalue 5e+01)) 9e+01))
  (return))