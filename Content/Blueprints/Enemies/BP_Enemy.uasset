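; Enemy actor for a spline-based shooter that moves, fires bullet spawners and reports play volume entry, exit and death to the GameState.
; Tagged movement components swap as the play volume reaches ActivationDistance or its bounds overlap PlayEntrySphere.
; Damage drives a decaying material hit flash, awards player Itano ammo by damage type, and triggers death effects.
; Construction previews the activation point on the spline and marks radar-tagged primitives via custom depth stencil.
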(event OnComponentEndOverlap(PlayEntrySphere)
  (params (OverlappedComponent :type Primitive%20Component%20Object%20Reference) (OtherActor :type Actor%20Object%20Reference) (OtherComp :type Primitive%20Component%20Object%20Reference) (OtherBodyIndex :type Integer))
  ;[1 1 1] Activate/deactivate bullet spawners and attach/detach on play volume entry/exit
  (Utilities|HandleComponentEndOverlap OtherComp))

(event OnComponentBeginOverlap(PlayEntrySphere)
  (params (OverlappedComponent :type Primitive%20Component%20Object%20Reference) (OtherActor :type Actor%20Object%20Reference) (OtherComp :type Primitive%20Component%20Object%20Reference) (OtherBodyIndex :type Integer) (bFromSweep :type Boolean) (SweepResult :type Hit%20Result%20Structure%20%28by%20ref%29))
  ;[1 1 1] Activate/deactivate bullet spawners and attach/detach on play volume entry/exit
  (Utilities|HandleComponentBeginOverlap OtherComp))

(event Custom|Event%20ActivateBullets
  (for _array_element (Actor|GetComponentsByClass "/Game/Blueprints/Components/BP_BulletSpawnerComponent.BP_BulletSpawnerComponent_C")
    (Components|Activation|Activate _array_element false)))

(event Custom|Event%20DeactivateBullets
  (for _array_element (Actor|GetComponentsByClass "/Game/Blueprints/Components/BP_BulletSpawnerComponent.BP_BulletSpawnerComponent_C")
    (Components|Activation|Deactivate _array_element)))

(event Game|Damage|EventAnyDamage
  (params (Damage :type Float%20%28single-precision%29) (DamageType :type Damage%20Type%20Object%20Reference) (InstigatedBy :type Controller%20Object%20Reference) (DamageCauser :type Actor%20Object%20Reference))
  (CallFunction|TakeDamage Damage DamageType))

(event EventTick
  (params (DeltaSeconds :type Float%20%28single-precision%29))
  (Utilities|FlowControl|Sequence
    (:then_0
      ;[1 1 1] Reduce hit flash intensity
      (for _array_element (Variables|State|GetDynamicMaterialInstances)
        (Utilities|IsValid _array_element
          (:Is%20Valid
            (Rendering|Material|SetScalarParameterValue _array_element "HitFlashEmissive" (Variables|State|GetCurrentHitFlashIntensity) :!class /Script/Engine.MaterialInstanceDynamic))))
      (Variables|State|SetCurrentHitFlashIntensity (* (Variables|State|GetCurrentHitFlashIntensity) 0.5)))
    (:then_1
      (if (>= (Variables|/Game/Blueprints/Game/BP_PlayVolume.BP_PlayVolume_C|GetDistanceAlongSpline (CallFunction|GetPlayVolume)) (Variables|Stats|Movement|GetActivationDistance))
        (Utilities|FlowControl|DoOnce false
          (:Completed
            (Utilities|SwitchMovementComponent (Variables|Stats|Movement|GetActivationMovementComponent))))))))

(event EventMatchStarted
  (CallFunction|InitializeEnemy))

(fn ConstructionScript
  (bind _returnvalue (Actor|GetComponentsbyTag "/Script/Shmup3D.S3DEnemyMovementComponent" "PlayEntryMovement"))
  (bind _returnvalue_2 (Actor|GetComponentsbyTag "/Script/Shmup3D.S3DEnemyMovementComponent" "PlayExitMovement"))
  (bind _returnvalue_3 (Actor|GetComponentsbyTag "/Script/Shmup3D.S3DEnemyMovementComponent" "InitialMovement"))
  (bind _returnvalue_4 (Actor|GetComponentsbyTag "/Script/Shmup3D.S3DEnemyMovementComponent" "ActivationMovement"))
  (bind _activationindicatorsphere (Variables|Default|GetActivationIndicatorSphere))
  (Utilities|FlowControl|Sequence
    (:then_0
      (if (> (Utilities|Array|Length _returnvalue_3) 0)
        (Variables|Stats|Movement|SetInitialMovementComponent (Utilities|Array|Get(acopy) _returnvalue_3))))
    (:then_1
      (if (> (Utilities|Array|Length _returnvalue_4) 0)
        (Variables|Stats|Movement|SetActivationMovementComponent (Utilities|Array|Get(acopy) _returnvalue_4))))
    (:then_2
      (if (> (Utilities|Array|Length _returnvalue) 0)
        (Variables|Stats|Movement|SetPlayEntryMovementComponent (Utilities|Array|Get(acopy) _returnvalue))))
    (:then_3
      (if (> (Utilities|Array|Length _returnvalue_2) 0)
        (Variables|Stats|Movement|SetPlayExitMovementComponent (Utilities|Array|Get(acopy) _returnvalue_2))))
    (:then_4
      (bind _outactors (Actor|GetAllActorsOfClass "/Game/Blueprints/Environment/BP_PlayVolumePath.BP_PlayVolumePath_C"))
      (if (and (> (Utilities|Array|Length _outactors) 0) (>= (Variables|Stats|Movement|GetActivationDistance) 0.0))
        (Transformation|SetWorldLocation _activationindicatorsphere (Spline|GetLocationatDistanceAlongSpline (Variables|/Game/Blueprints/Environment/BP_SplineActor.BP_SplineActor_C|GetSpline (Utilities|Array|Get(acopy) _outactors)) (Variables|Stats|Movement|GetActivationDistance) "World") false true)
        (else
          (Rendering|SetVisibility _activationindicatorsphere false true))))
    (:then_5
      (for _array_element (Actor|GetComponentsbyTag "/Script/Engine.PrimitiveComponent" "ShowOnRadar")
        (Rendering|SetRenderCustomDepth _array_element true)
        (Rendering|SetCustomDepthStencilValue _array_element 255)))))

(fn RefillItanoAmmo
  (params (Amount :type Integer))
  (return))

(fn EnemyDeath
  (CallFunction|PlayDeathEffects)
  (CallFunction|RemoveSelffromPlay)
  (Actor|DestroyActor)
  (return))

(fn PlayDeathEffects
  (bind _returnvalue (Transformation|GetActorLocation))
  (Effects|SpawnEmitteratLocation (Variables|Stats|Effects|GetDeathParticleSystem) _returnvalue (Transformation|GetActorRotation))
  (Audio|PlaySoundatLocation (Variables|Stats|Effects|GetDeathSound) _returnvalue)
  (return))

(fn RemoveSelffromPlay
  (Default|RemoveEnemyfromPlay (CallFunction|GetGameState) self)
  (return))

(fn TakeDamage
  (params (Damage :type Float%20%28single-precision%29) (DamageType :type Damage%20Type%20Object%20Reference))
  (bind _playerstate (CallFunction|GetPlayerState))
  (if (> (Variables|Stats|Lifecycle|GetHealth) 0)
    (Utilities|FlowControl|Sequence
      (:then_0
        ;[1 1 1] Damage Handler
        (Variables|State|SetCurrentHitFlashIntensity 1e+01)
        (Variables|Stats|Lifecycle|SetHealth (- (Variables|Stats|Lifecycle|GetHealth) (Math|Float|Round Damage)))
        (Audio|PlaySoundatLocation (Variables|Stats|Effects|GetDamageSound) (Transformation|GetActorLocation)))
      (:then_1
        (bind _ass3ddamage_type (Utilities|Casting|CastToS3DDamageType DamageType))
        (Default|GiveItanoAmmo _playerstate (Variables|/Script/Shmup3D.S3DDamageType|GetItanoRefillOnHit _ass3ddamage_type))
        (if (and (Variables|/Script/Shmup3D.S3DDamageType|GetbRefillItanoAmmoOnKill _ass3ddamage_type) (<= (Variables|Stats|Lifecycle|GetHealth) 0))
          (Default|GiveItanoAmmo _playerstate (Variables|Stats|Lifecycle|GetItanoRefillOnDeath))))
      (:then_2
        (if (<= (Variables|Stats|Lifecycle|GetHealth) 0)
          (CallFunction|EnemyDeath)))
      (:then_3
        (return)))
    (else
      (return))))

(fn EnterPlayVolume
  (if (Variables|Stats|Bullets|GetActivateBulletsOnPlayVolumeEntry)
    (CallFunction|EventActivateBullets))
  (Utilities|SwitchMovementComponent (Variables|Stats|Movement|GetPlayEntryMovementComponent)
    (:Exec%20Out
      (Default|EnemyEnteredPlayVolume (CallFunction|GetGameState) self)
      (return))))

(fn LeavePlayVolume
  (CallFunction|EventDeactivateBullets)
  (Utilities|SwitchMovementComponent (Variables|Stats|Movement|GetPlayExitMovementComponent)
    (:Exec%20Out
      (if (> (Variables|Stats|Lifecycle|GetHealth) 0)
        (Default|EnemyLeftPlayVolume (CallFunction|GetGameState) self)))))

(fn InitializeEnemy
  (Utilities|FlowControl|Sequence
    (:then_0
      ;[1 1 1] Create dynamic materials for hit flash
      (for _array_element (Actor|GetComponentsByClass "/Script/Engine.PrimitiveComponent")
        (Utilities|IsValid (Rendering|Material|GetMaterial _array_element 0)
          (:Is%20Valid
            (bind _returnvalue (Rendering|Material|CreateDynamicMaterialInstance _array_element 0 (Rendering|Material|GetMaterial _array_element 0) :!class /Script/Engine.PrimitiveComponent))
            (Utilities|Array|Add (Variables|State|GetDynamicMaterialInstances) _returnvalue)))))
    (:then_1
      (for _array_element_2 (Actor|GetComponentsByClass "/Game/Blueprints/Components/BP_BulletSpawnerComponent.BP_BulletSpawnerComponent_C")
        (Default|Initialize _array_element_2)))
    (:then_2
      (Utilities|TrySetMovementComponentActive (Variables|Stats|Movement|GetInitialMovementComponent) true))
    (:then_3
      (for _array_element_3 (Class|PrimitiveComponent|GetOverlappingComponents (Variables|Default|GetPlayEntrySphere))
        (Utilities|HandleComponentBeginOverlap _array_element_3)))))